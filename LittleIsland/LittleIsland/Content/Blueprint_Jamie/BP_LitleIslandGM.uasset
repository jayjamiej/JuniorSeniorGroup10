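; Game mode for a tile-based, turn-based game that spawns three player characters and cycles turns between them.
; Match start is held until the navigation manager reports its tiles spawned, plus a short delay.
; Pawn spawning possesses an ambient camera and places characters on the start locator's tile and two adjacent tiles.
; After a match state change, each AI controller's turn-complete event advances the turn and switches the player controller's active character.
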(event `self.ReceiveBeginPlay`
  (bind _outactors (`GameplayStatics.GetAllActorsOfClass` "/Game/Blueprint_Jamie/BP_NavigationManager.BP_NavigationManager_C"))
  (bind _output (`|GetArrayItem` _outactors))
  (add `/Game/Blueprint_Jamie/BP_NavigationManager.TilesSpawned` _output (delegate `ReadyToSpawn`))
  (`/Game/Blueprint_Jamie/BP_NavigationManager.Init` _output))

(event `ReadyToSpawn`
  (`KismetSystemLibrary.Delay` 0.5)
  (set `self.TilesSpawned` true))

(event `self.K2_OnSetMatchState`
  (params (NewState :type Name))
  (switch `name` NewState
    (:`inProgress`
      (`KismetSystemLibrary.Delay` 1.0)
      (`self.InitTurns`))))

(event `InitTurns`
  (bind _values (`BlueprintMapLibrary.Map_Values` (`self.PlayerCharacters`)))
  (for _array_element _values
    (add `/Game/Blueprint_Jamie/Characters/BP_AiCharControl.onTurnComplete` (`/Game/Blueprints/BP_Character.AiController` _array_element) (delegate `EndTurn`)))
  (bind _output_get (set `self.CurrentTurn` 1))
  (`self.StartTurn` _output_get))

(event `EndTurn`
  (bind _returnvalue (+ (`self.CurrentTurn`) 1))
  (bind _output_get (set `self.CurrentTurn` (select `bool` (> _returnvalue (`self.maxTurns`)) :`false` _returnvalue :`true` 1)))
  (`self.StartTurn` _output_get))

(event `StartTurn`
  (params (CharacterID :type Integer))
  (bind _output_get (set `self.ActiveCharacter` (`BlueprintMapLibrary.Map_Find` (`self.PlayerCharacters`) CharacterID)))
  (`/Game/Blueprint_Jamie/BP_PlayerController.SwitchCharacter` (`self.PlayerController`) _output_get))

(fn `FindPlayerStart`
  (params (Player :type "Controller Object Reference") (IncomingName :type String))
  (returns (ReturnValue :type "Actor Object Reference"))
  (bind _outactors (`GameplayStatics.GetAllActorsOfClass` "/Game/Blueprint_Jamie/BP_PlayerSpawnLocator.BP_PlayerSpawnLocator_C"))
  (for _array_element _outactors
    (if (`/Game/Blueprint_Jamie/BP_PlayerSpawnLocator.InitSpawn` _array_element)
      (return _array_element)))
  (return null))

(fn `ReadyToStartMatch`
  (returns (ReturnValue :type Boolean))
  (return (`self.TilesSpawned`)))

(fn `SpawnDefaultPawnFor`
  (params (NewPlayer :type "Controller Object Reference") (StartSpot :type "Actor Object Reference"))
  (returns (ReturnValue :type "Pawn Object Reference"))
  (bind _controller (message `/Game/Blueprint_Jamie/iRef.getPlayerController` NewPlayer))
  (bind _output_get (set `self.PlayerController` _controller))
  (bind _returnvalue (`|SpawnActorFromClass` "/Game/Blueprint_Jamie/BP_AmbientCamera.BP_AmbientCamera_C" (`KismetMathLibrary.MakeTransform` (0.0 0.0 0.0)) "Undefined" "OverrideRootScale" null null))
  (`Controller.Possess` _output_get _returnvalue)
  (bind _locator (message `/Game/Blueprint_Jamie/iRef.getSpawnLocator` StartSpot))
  (`|ExecutionSequence`
    (:`then_0`
      (bind _spawntile (`/Game/Blueprint_Jamie/BP_PlayerSpawnLocator.SpawnTile` _locator))
      (bind _returnvalue_2 (`|SpawnActorFromClass` "/Game/Blueprints/BP_Character.BP_Character_C" (`KismetMathLibrary.MakeTransform` (+ (`SceneComponent.K2_GetComponentLocation` (`/Game/Blueprint_Jamie/BP_NavigationTile.TileLocator` _spawntile)) (0.0 0.0 100.0))) "Undefined" "OverrideRootScale" null null))
      (`BlueprintMapLibrary.Map_Add` (`self.PlayerCharacters`) 1 _returnvalue_2)
      (`/Game/Blueprints/BP_Character.Init` _returnvalue_2 1))
    (:`then_1`
      (bind _returnvalue_3 (`|SpawnActorFromClass` "/Game/Blueprints/BP_Character.BP_Character_C" (`KismetMathLibrary.MakeTransform` (+ (`SceneComponent.K2_GetComponentLocation` (`/Game/Blueprint_Jamie/BP_NavigationTile.TileLocator` (`/Game/Blueprint_Jamie/BP_NavigationTile.FindAdjacentTile` _spawntile "NewEnumerator1"))) (0.0 0.0 100.0))) "Undefined" "OverrideRootScale" null null))
      (`BlueprintMapLibrary.Map_Add` (`self.PlayerCharacters`) 2 _returnvalue_3)
      (`/Game/Blueprints/BP_Character.Init` _returnvalue_3 2))
    (:`then_2`
      (bind _returnvalue_4 (`|SpawnActorFromClass` "/Game/Blueprints/BP_Character.BP_Character_C" (`KismetMathLibrary.MakeTransform` (+ (`SceneComponent.K2_GetComponentLocation` (`/Game/Blueprint_Jamie/BP_NavigationTile.TileLocator` (`/Game/Blueprint_Jamie/BP_NavigationTile.FindAdjacentTile` _spawntile "NewEnumerator3"))) (0.0 0.0 100.0))) "Undefined" "OverrideRootScale" null null))
      (`BlueprintMapLibrary.Map_Add` (`self.PlayerCharacters`) 3 _returnvalue_4)
      (`/Game/Blueprints/BP_Character.Init` _returnvalue_4 3)
      (return null))))

(fn `UserConstructionScript`)