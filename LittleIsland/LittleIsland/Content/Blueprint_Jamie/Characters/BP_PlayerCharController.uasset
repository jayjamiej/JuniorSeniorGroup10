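; AI controller that moves a player character one step at a time across a tile grid.
; Init stores the character and passes itself back to it.
; MoveToTile picks one of four directions from the target's world offset, checking positive X, positive Y, then negative X before the fallback.
; MoveInDirection looks up that adjacent tile and calls MoveToLocation, with debug prints; GetNavTile is an empty stub.
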(event `Init`
  (params (Character :type "/Game/Blueprint_Jamie/Characters/TestCharacter Object Reference"))
  (bind _output_get (set `self.ControlledCharacter` Character))
  (`/Game/Blueprint_Jamie/Characters/TestCharacter.Init` _output_get self))

(event `MoveToTile`
  (params (Tile :type "/Game/Blueprint_Jamie/BP_NavigationTile Object Reference"))
  (bind _returnvalue (- (`SceneComponent.K2_GetComponentLocation` (`/Game/Blueprint_Jamie/BP_NavigationTile.TileLocator` (`self.TargetTile`))) (`SceneComponent.K2_GetComponentLocation` (`/Game/Blueprint_Jamie/BP_NavigationTile.TileLocator` (`/Game/Blueprint_Jamie/Characters/TestCharacter.CurrentLocation` (`self.ControlledCharacter`))))))
  (bind _x (.x _returnvalue))
  (set `self.TargetTile` Tile)
  (`KismetSystemLibrary.PrintString` (`KismetStringLibrary.Conv_VectorToString` _returnvalue))
  (if (> _x 0.0)
    (`self.MoveInDirection` "NewEnumerator0") ; North
    (elif (> (.y _returnvalue) 0.0)
      (`self.MoveInDirection` "NewEnumerator1") ; North
      (elif (< _x 0.0)
        (`self.MoveInDirection` "NewEnumerator2") ; North
        (else
          (`self.MoveInDirection` "NewEnumerator3") ; North
        )))))

(fn `getNavTile`
  (returns (NavTile :type "/Game/Blueprint_Jamie/BP_NavigationTile Object Reference"))
  (return null))

(fn `getPlayerAI_Controller`
  (returns (Controller :type "/Game/Blueprint_Jamie/Characters/BP_PlayerCharController Object Reference"))
  (return self))

(fn `MoveInDirection`
  (params (Key :type "/Game/Blueprint_Jamie/eCompass Enum" :default "NewEnumerator0"))
  (bind _returnvalue (`self.MoveToLocation` (`SceneComponent.K2_GetComponentLocation` (`/Game/Blueprint_Jamie/BP_NavigationTile.TileLocator` (`BlueprintMapLibrary.Map_Find` (`/Game/Blueprint_Jamie/BP_NavigationTile.AdjacentTiles` (`/Game/Blueprint_Jamie/Characters/TestCharacter.CurrentLocation` (`self.ControlledCharacter`))) Key))) 0.0 true true false true null))
  (`KismetSystemLibrary.PrintString` (`|GetEnumeratorNameAsString` _returnvalue)))

(fn `UserConstructionScript`)