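; AI controller that walks a turn-based character across a tile grid toward a target tile.
; A one-second looping timer tries directions chosen by the X/Y offset, cycling to others when blocked, and issues MoveToLocation to the adjacent tile.
; Each step spends an action point; at zero it deactivates the character, signals turn completion and stops the timer.
; SetActive refills points and activates the character; most getter functions are empty stubs.
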(event `Init`
  (params (Character :type "/Game/Blueprints/BP_Character Object Reference"))
  (set `self.ControlledCharacter` Character))

(event `MoveToTile`
  (params (Tile :type "/Game/Blueprint_Jamie/BP_NavigationTile Object Reference"))
  (set `self.TargetTile` Tile)
  (`self.MoveToNext`)
  (bind _returnvalue (`KismetSystemLibrary.K2_SetTimerDelegate` (delegate `MoveToNext`) 1.0 true))
  (set `self.MoveTimer` _returnvalue))

(event `CancelMovement`
  (`KismetSystemLibrary.K2_ClearAndInvalidateTimerHandle` (`self.MoveTimer`)))

(event `MoveToNext`
  (bind _location (`/Game/Blueprint_Jamie/BP_NavigationTile.GetTileLocation` (`self.TargetTile`)))
  (bind _location_2 (`/Game/Blueprint_Jamie/BP_NavigationTile.GetTileLocation` (`/Game/Blueprints/BP_Character.CurrentLocation` (`self.ControlledCharacter`))))
  (bind _x (.x (- _location _location_2)))
  (if (== _location_2 _location)
    (`KismetSystemLibrary.K2_ClearAndInvalidateTimerHandle` (`self.MoveTimer`))
    (elif (> _x 0.0)
      (bind _success (`self.MoveInDirection` "NewEnumerator0" :!label _label)) ; North
      (if (not _success)
        (if (> (.y (- _location _location_2)) 0.0) :!label _label_2
          (bind _success_2 (`self.MoveInDirection` "NewEnumerator1")) ; North
          (if (not _success_2)
            (if (< _x 0.0) :!label _label_3
              (bind _success_3 (`self.MoveInDirection` "NewEnumerator2")) ; North
              (if (not _success_3)
                (bind _success_4 (`self.MoveInDirection` "NewEnumerator3" :!label _label_4)) ; North
                (if (not _success_4)
                  (goto _label)))
              (else
                (goto _label_4))))
          (else
            (goto _label_3))))
      (else
        (goto _label_2)))))

(event `SetActive`
  (params (Controller :type "/Game/Blueprint_Jamie/BP_PlayerController Object Reference"))
  (set `self.IsActive` false)
  (set `self.ActionPoints` (`self.MaxActionPoints`))
  (`/Game/Blueprints/BP_Character.ActivateCharacter` (`self.ControlledCharacter`) Controller))

(fn `getCharacter`
  (returns (Character :type "/Game/Blueprints/BP_Character Object Reference"))
  (return null))

(fn `getNavTile`
  (returns (NavTile :type "/Game/Blueprint_Jamie/BP_NavigationTile Object Reference"))
  (return null))

(fn `getPlayerAI_Controller`
  (returns (Controller :type "/Game/Blueprint_Jamie/Characters/BP_AiCharControl Object Reference"))
  (return self))

(fn `getPlayerController`
  (returns (Controller :type "/Game/Blueprint_Jamie/BP_PlayerController Object Reference"))
  (return null))

(fn `getSpawnLocator`
  (returns (Locator :type "/Game/Blueprint_Jamie/BP_PlayerSpawnLocator Object Reference"))
  (return null))

(fn `MoveInDirection`
  (params (Key :type "/Game/Blueprint_Jamie/eCompass Enum" :default "NewEnumerator0"))
  (returns (Success :type Boolean))
  (bind (_location _canmove) (`/Game/Blueprint_Jamie/BP_NavigationTile.GetTileLocationForMove` (`BlueprintMapLibrary.Map_Find` (`/Game/Blueprint_Jamie/BP_NavigationTile.AdjacentTiles` (`/Game/Blueprints/BP_Character.CurrentLocation` (`self.ControlledCharacter`))) Key)))
  (if _canmove
    (`self.MoveToLocation` _location -1.0 false true false true null)
    (`self.SubtractActionPoint`)
    (`KismetSystemLibrary.PrintString` "Hello")
    (return true)
    (else
      (return false))))

(fn `SubtractActionPoint`
  (bind _output_get (set `self.ActionPoints` (- (`self.ActionPoints`) 1)))
  (`KismetSystemLibrary.PrintString` (`KismetStringLibrary.Conv_IntToString` _output_get))
  (if (== _output_get 0)
    (`/Game/Blueprints/BP_Character.DeactivateCharacter` (`self.ControlledCharacter`))
    (`self.onTurnComplete`)
    (`KismetSystemLibrary.K2_ClearAndInvalidateTimerHandle` (`self.MoveTimer`))))

(fn `UserConstructionScript`)