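; BP_NavigationTile is a tile for grid-based character movement that passes itself to a controller's MoveCharacterTo when clicked.
; On Init it destroys itself if off the navmesh, otherwise waits briefly and box-traces four sides to map neighboring tiles by direction, resolved through interface messages.
; It tracks occupancy to report whether it can be moved onto, and swaps plane materials for hover and active-direction highlights.
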(event `Directions`
  (params (Active :type Boolean))
  (bind _plane (`self.Plane`))
  (if Active
    (set `self.DirectionActive` true)
    (if (not (`self.Occupied`))
      (`PrimitiveComponent.SetMaterial` _plane 0 "/Game/RedSquare.RedSquare"))
    (else
      (set `self.DirectionActive` false)
      (`PrimitiveComponent.SetMaterial` _plane 0 "/Game/UI_Square_Mat.UI_Square_Mat"))))

(event `Init`
  (if (`.ReturnValue` (`NavigationSystemV1.K2_ProjectPointToNavigation` (`NavigationSystemV1.GetNavigationSystem`) (`self.K2_GetActorLocation`) null null (0.0 0.0 0.0)))
    (`KismetSystemLibrary.Delay` 0.01)
    (`self.DetectAdjacent`)
    (else
      (`self.K2_DestroyActor`))))

(event `/Game/Blueprint_Jamie/iMouse.MouseHover`
  (`PrimitiveComponent.SetMaterial` (`self.Plane`) 0 "/Game/GreenSquare.GreenSquare"))

(event `/Game/Blueprint_Jamie/iMouse.MouseUnhover`
  (bind _plane (`self.Plane`))
  (if (`self.DirectionActive`)
    (`PrimitiveComponent.SetMaterial` _plane 0 "/Game/RedSquare.RedSquare")
    (else
      (`PrimitiveComponent.SetMaterial` _plane 0 "/Game/UI_Square_Mat.UI_Square_Mat"))))

(event `/Game/Blueprint_Jamie/iMouse.MouseClick`
  (params (Controller :type "/Game/Blueprint_Jamie/BP_PlayerController Object Reference"))
  (`/Game/Blueprint_Jamie/BP_PlayerController.MoveCharacterTo` Controller self))

(event `DetectAdjacent`
  (bind _returnvalue (`SceneComponent.K2_GetComponentLocation` (`self.TileLocator`)))
  (for _array_element (`|MakeArray` "NewEnumerator0" "NewEnumerator1" "NewEnumerator2" "NewEnumerator3" :!type "/Game/Blueprint_Jamie/eCompass Enum")
    (bind _value (`BlueprintMapLibrary.Map_Find` (`|MakeMap` "NewEnumerator0" (+ _returnvalue (75.0 0.0 50.0)) "NewEnumerator1" (+ _returnvalue (0.0 75.0 50.0)) "NewEnumerator2" (+ _returnvalue (-75.0 0.0 50.0)) "NewEnumerator3" (+ _returnvalue (0.0 -75.0 50.0)) :!type "/Game/Blueprint_Jamie/eCompass Enum") _array_element))
    (bind (_outhit _returnvalue_2) (`KismetSystemLibrary.BoxTraceSingleForObjects` :`Start` _value :`End` (+ _value (0.0 0.0 1.0)) :`HalfSize` (25.0 25.0 25.0) :`ObjectTypes` (`|MakeArray` "ObjectTypeQuery7" :!type "EObjectTypeQuery Enum") :`DrawTime` 1.0))
    (if _returnvalue_2
      (`self.AddAdjacent` _array_element (`.HitActor` (`GameplayStatics.BreakHitResult` _outhit))))))

(fn `AddAdjacent`
  (params (Direction :type "/Game/Blueprint_Jamie/eCompass Enum" :default "NewEnumerator0") (Actor :type "Actor Object Reference"))
  (returns (Success :type Boolean))
  (bind _navtile (message `/Game/Blueprint_Jamie/iRef.getNavTile` Actor))
  (`/Engine/EditorBlueprintResources/StandardMacros.IsValid` _navtile
    (:`Is Valid`
      (`BlueprintMapLibrary.Map_Add` (`self.AdjacentTiles`) Direction _navtile)
      (return true))
    (:`Is Not Valid`
      (return false))))

(fn `FindAdjacentTile`
  (params (Direction :type "/Game/Blueprint_Jamie/eCompass Enum" :default "NewEnumerator0"))
  (returns (Tile :type "/Game/Blueprint_Jamie/BP_NavigationTile Object Reference"))
  (return (`BlueprintMapLibrary.Map_Find` (`self.AdjacentTiles`) Direction)))

(fn `getCharacter`
  (returns (Character :type "/Game/Blueprints/BP_Character Object Reference"))
  (return null))

(fn `getNavTile`
  (returns (NavTile :type "/Game/Blueprint_Jamie/BP_NavigationTile Object Reference"))
  (return self))

(fn `getPlayerAI_Controller`
  (returns (Controller :type "/Game/Blueprint_Jamie/Characters/BP_AiCharControl Object Reference"))
  (return null))

(fn `getPlayerController`
  (returns (Controller :type "/Game/Blueprint_Jamie/BP_PlayerController Object Reference"))
  (return null))

(fn `getSpawnLocator`
  (returns (Locator :type "/Game/Blueprint_Jamie/BP_PlayerSpawnLocator Object Reference"))
  (return null))

(fn `GetTileLocation`
  (returns (Location :type "Vector Structure"))
  (return (`SceneComponent.K2_GetComponentLocation` (`self.TileLocator`))))

(fn `GetTileLocationForMove`
  (returns (Location :type "Vector Structure") (CanMove :type Boolean))
  (return (`SceneComponent.K2_GetComponentLocation` (`self.TileLocator`)) (not (`self.Occupied`))))

(fn `SetOccupied`
  (params (occupied :type Boolean))
  (set `self.Occupied` occupied))

(fn `UserConstructionScript`)