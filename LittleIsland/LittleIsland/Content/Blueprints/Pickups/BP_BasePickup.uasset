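; Base pickup actor for a tile-based game with action points, collected by clicking from an adjacent tile.
; On its first valid box overlap with a nav tile, it snaps to that tile and marks it occupied.
; Hover swaps the cube material to green.
; A click when adjacent spends an action point, passes the pickup to the controller, frees the tile and destroys the actor.
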(event `self.Box.OnComponentBeginOverlap`
  (params (OverlappedComponent :type "PrimitiveComponent Object Reference") (OtherActor :type "Actor Object Reference") (OtherComp :type "PrimitiveComponent Object Reference") (OtherBodyIndex :type Integer) (bFromSweep :type Boolean) (SweepResult :type "HitResult Structure (by ref)"))
  (bind _navtile (message `/Game/Blueprints/Interfaces/iRef.getNavTile` OtherActor))
  (`/Engine/EditorBlueprintResources/StandardMacros.IsValid` _navtile
    (:`Is Valid`
      (`/Engine/EditorBlueprintResources/StandardMacros.DoOnce` false
        (:`Completed`
          (bind _output_get (set `self.Location` _navtile))
          (`/Game/Blueprints/Navigation/BP_NavigationTile.SetOccupied` _output_get true)
          (`self.K2_SetActorLocation` (`/Game/Blueprints/Navigation/BP_NavigationTile.GetTileLocation` _output_get)))))))

(event `/Game/Blueprints/Interfaces/iMouse.MouseHover`
  (`PrimitiveComponent.SetMaterial` (`self.Cube`) 0 "/Game/Assets/MaterialTemp/M_Green.M_Green"))

(event `/Game/Blueprints/Interfaces/iMouse.MouseUnhover`
  (`PrimitiveComponent.SetMaterial` (`self.Cube`) 0 "/Engine/BasicShapes/BasicShapeMaterial.BasicShapeMaterial"))

(event `/Game/Blueprints/Interfaces/iMouse.MouseClick`
  (params (Controller :type "/Game/Blueprints/Navigation/BP_PlayerControl_PC Object Reference"))
  (bind _atlocation (`/Game/Blueprints/Navigation/BP_NavigationTile.CheckIsAdjacent` (`/Game/Blueprints/Navigation/BP_PlayerControl_PC.getCurrentCharacterTile` Controller) (`self.Location`)))
  (if _atlocation
    (`/Game/Blueprints/Characters/BP_AiPlayerController_AI.SubtractActionPoint` (`/Game/Blueprints/Navigation/BP_PlayerControl_PC.getAI` Controller))
    (`/Game/Blueprints/Navigation/BP_PlayerControl_PC.PickupObject` Controller self)
    (`/Game/Blueprints/Navigation/BP_NavigationTile.SetOccupied` (`self.Location`) false)
    (`self.K2_DestroyActor`)))

(fn `CheckLocation`
  (params (Controller :type "/Game/Blueprints/Navigation/BP_PlayerControl_PC Object Reference"))
  (returns (ReturnValue :type Boolean))
  (bind _tiles (`/Game/Blueprints/Navigation/BP_NavigationTile.GetAllAdjacent` (`/Game/Blueprints/Navigation/BP_PlayerControl_PC.getCurrentCharacterTile` Controller)))
  (for _array_element _tiles
    (if (== _array_element (`self.Location`))
      (return true)))
  (return false))

(fn `UserConstructionScript`)