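; Base enemy for tile-based combat that takes damage, burns, dies and serves as a mouse-click attack target.
; It snaps to the first nav tile it overlaps, marking it occupied until death.
; Damage plays a timeline hop and deducts health; burn damage also starts timed fire ticks at half damage.
; Hover turns it red, clicks trigger the controller's AI attack if adjacent, and death plays a fall before destruction.
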(event `self.ReceiveAnyDamage`
  (params (Damage :type "Float (single-precision)") (DamageType :type "DamageType Object Reference") (InstigatedBy :type "Controller Object Reference") (DamageCauser :type "Actor Object Reference"))
  (`self.DamageHop`)
  (bind _output_get (set `self.DamageAmount` Damage))
  (`self.DeductHealth` _output_get)
  (if (== (`GameplayStatics.GetObjectClass` DamageType) "/Game/Blueprints/DamageTypes/BP_Burn_DT.BP_Burn_DT_C")
    (set `self.BurnDamage` (/ (`self.DamageAmount`) 2.0))
    (`self.StartBurn`)))

(event `DamageHop`
  (bind (_direction _alpha) (`Timeline|Hop` :!via `PlayFromStart`)
    (:`Update`
      (`SceneComponent.K2_SetRelativeLocation` (`self.Mesh`) (`KismetMathLibrary.VLerp` (0.0 0.0 -90.0) (0.0 0.0 -40.0) _alpha) false false))))

(event `StartBurn`
  (bind _returnvalue (`KismetSystemLibrary.K2_SetTimerDelegate` (delegate `Burn`) 1.5 true))
  (bind _output_get (set `self.BurnTimer` _returnvalue))
  (`KismetSystemLibrary.K2_SetTimerDelegate` (delegate `BurnStop`) 10.0))

(event `BurnStop`
  (`KismetSystemLibrary.K2_ClearAndInvalidateTimerHandle` (stale `StartBurn` _output_get)))

(event `Burn`
  (`GameplayStatics.SpawnEmitterAtLocation` "/Game/Assets/PS_Fire.PS_Fire" (`SceneComponent.K2_GetComponentLocation` (`self.CapsuleComponent`)))
  (`self.DeductHealth` (`self.BurnDamage`)))

(event `self.CapsuleComponent.OnComponentBeginOverlap`
  (params (OverlappedComponent :type "PrimitiveComponent Object Reference") (OtherActor :type "Actor Object Reference") (OtherComp :type "PrimitiveComponent Object Reference") (OtherBodyIndex :type Integer) (bFromSweep :type Boolean) (SweepResult :type "HitResult Structure (by ref)"))
  (bind _navtile (message `/Game/Blueprints/Interfaces/iRef.getNavTile` OtherActor))
  (`/Engine/EditorBlueprintResources/StandardMacros.IsValid` _navtile
    (:`Is Valid`
      (`/Engine/EditorBlueprintResources/StandardMacros.DoOnce` false
        (:`Completed`
          (bind _output_get (set `self.Location` _navtile))
          (`/Game/Blueprints/Navigation/BP_NavigationTile.SetOccupied` _output_get true)
          (`self.K2_SetActorLocation` (`/Game/Blueprints/Navigation/BP_NavigationTile.GetTileLocation` _output_get)))))))

(event `Death`
  (bind _burntimer (`self.BurnTimer`))
  (if (`KismetSystemLibrary.K2_IsValidTimerHandle` _burntimer)
    (`KismetSystemLibrary.K2_ClearAndInvalidateTimerHandle` _burntimer)
    (bind (_direction _alpha) (`Timeline|DeathMove` :!label _label)
      (:`Update`
        (`SceneComponent.K2_SetRelativeTransform` (`self.Mesh`) (`KismetMathLibrary.TLerp` (`KismetMathLibrary.MakeTransform` (0.0 0.0 -90.0) (struct :`Yaw` -90.0)) (`KismetMathLibrary.MakeTransform` (83.0 0.0 -80.0) (struct :`Yaw` -90.0 :`Roll` -80.0)) _alpha) false false))
      (:`Finished`
        (`KismetSystemLibrary.Delay` 0.5)
        (`/Game/Blueprints/Navigation/BP_NavigationTile.SetOccupied` (`self.Location`) false)
        (`self.K2_DestroyActor`)))
    (else
      (goto _label))))

(event `/Game/Blueprints/Interfaces/iMouse.MouseHover`
  (bind _mesh (`self.Mesh`))
  (`PrimitiveComponent.SetMaterial` _mesh 0 "/Game/Assets/MaterialTemp/M_Red.M_Red")
  (`PrimitiveComponent.SetMaterial` _mesh 1 "/Game/Assets/MaterialTemp/M_Red.M_Red"))

(event `/Game/Blueprints/Interfaces/iMouse.MouseUnhover`
  (bind _mesh (`self.Mesh`))
  (`PrimitiveComponent.SetMaterial` _mesh 0 "/Game/Assets/AnimTemp/MCO_Mocap_Basics/Character/Materials/M_UE4Man_Body.M_UE4Man_Body")
  (`PrimitiveComponent.SetMaterial` _mesh 1 "/Game/Assets/AnimTemp/MCO_Mocap_Basics/Character/Materials/M_UE4Man_ChestLogo.M_UE4Man_ChestLogo"))

(event `/Game/Blueprints/Interfaces/iMouse.MouseClick`
  (params (Controller :type "/Game/Blueprints/Navigation/BP_PlayerControl_PC Object Reference"))
  (bind _atlocation (`/Game/Blueprints/Navigation/BP_NavigationTile.CheckIsAdjacent` (`/Game/Blueprints/Navigation/BP_PlayerControl_PC.getCurrentCharacterTile` Controller) (`self.Location`)))
  (if _atlocation
    (`/Game/Blueprints/Characters/BP_AiPlayerController_AI.Attack` (`/Game/Blueprints/Navigation/BP_PlayerControl_PC.getAI` Controller) self)))

(fn `DeductHealth`
  (params (ToDeduct :type "Float (double-precision)"))
  (bind _output_get (set `self.Health` (- (`self.Health`) ToDeduct)))
  (if (<= _output_get 0.0)
    (`self.Death`)))

(fn `UserConstructionScript`)