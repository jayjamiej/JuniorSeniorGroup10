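; BP_PlayerSpawnLocator is a navigation actor that records the nav tile at a player spawn location.
; On the first capsule overlap, gated by a DoOnce, it sends a GetNavTile message to the other actor and stores the result as SpawnTile.
; It exposes a set of getters for character, tile, controllers and locator, of which only GetSpawnLocator returns something, itself; the rest are empty stubs.
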(event `self.Capsule.OnComponentBeginOverlap`
  (params (OverlappedComponent :type "PrimitiveComponent Object Reference") (OtherActor :type "Actor Object Reference") (OtherComp :type "PrimitiveComponent Object Reference") (OtherBodyIndex :type Integer) (bFromSweep :type Boolean) (SweepResult :type "HitResult Structure (by ref)"))
  (`/Engine/EditorBlueprintResources/StandardMacros.DoOnce` false
    (:`Completed`
      (bind _navtile (message `/Game/Blueprints/Interfaces/iRef.getNavTile` OtherActor))
      (set `self.SpawnTile` _navtile))))

(fn `getCharacter`
  (returns (Character :type "/Game/Blueprints/Characters/BP_BasePlayer_Char Object Reference"))
  (return null))

(fn `getNavTile`
  (returns (NavTile :type "/Game/Blueprints/Navigation/BP_NavigationTile Object Reference"))
  (return null))

(fn `getPlayerAI_Controller`
  (returns (Controller :type "/Game/Blueprints/Characters/BP_AiPlayerController_AI Object Reference"))
  (return null))

(fn `getPlayerController`
  (returns (Controller :type "/Game/Blueprints/Navigation/BP_PlayerControl_PC Object Reference"))
  (return null))

(fn `getSpawnLocator`
  (returns (Locator :type "/Game/Blueprints/Navigation/BP_PlayerSpawnLocator Object Reference"))
  (return self))

(fn `UserConstructionScript`)