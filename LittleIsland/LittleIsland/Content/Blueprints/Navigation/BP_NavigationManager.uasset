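; Navigation manager that fills a rectangular area with a grid of BP_NavigationTile actors.
; The construction script sizes the box from NavDimensions rounded to 100-unit steps and insets TopLeft and BottomRight markers by half a tile.
; Init, rather than BeginPlay, spawns and initializes tiles row by row along world X from TopLeft, wrapping at BottomRight's X, then calls TilesSpawned.
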(event `self.ReceiveBeginPlay`)

(event `Init`
  (`self.SpawnNav`))

(fn `SpawnNav`
  (locals (LastLocation :type "Vector Structure"))
  (bind (_navdimensions_x _navdimensions_y) (`KismetMathLibrary.BreakVector2D` (`self.NavDimensions`)))
  (bind _lastlocation (`local.LastLocation`))
  (bind (_lastlocation_x _lastlocation_y _lastlocation_z) (`KismetMathLibrary.BreakVector` (`local.LastLocation`)))
  (bind _returnvalue_x (`KismetMathLibrary.BreakVector` (`SceneComponent.K2_GetComponentLocation` (`self.TopLeft`))))
  (bind _returnvalue_x_2 (`KismetMathLibrary.BreakVector` (`SceneComponent.K2_GetComponentLocation` (`self.BottomRight`))))
  (for _index (range 1 (+ (`KismetMathLibrary.FTrunc` (* (/ _navdimensions_x 100.0) (/ _navdimensions_y 100.0))) 1))
    (bind _output_get (set `local.LastLocation` (select `bool` (== _index 1) :`false` (select `bool` (== (.x _lastlocation) _returnvalue_x_2) :`false` (+ _lastlocation (100.0 0.0 0.0)) :`true` (`KismetMathLibrary.MakeVector` _returnvalue_x (+ _lastlocation_y 100.0) _lastlocation_z)) :`true` (`SceneComponent.K2_GetComponentLocation` (`self.TopLeft`)))))
    (bind _returnvalue (`|SpawnActorFromClass` "/Game/Blueprints/Navigation/BP_NavigationTile.BP_NavigationTile_C" (`KismetMathLibrary.MakeTransform` _output_get) "Undefined" "OverrideRootScale" null null))
    (`/Game/Blueprints/Navigation/BP_NavigationTile.Init` _returnvalue))
  (`self.TilesSpawned`))

(fn `UserConstructionScript`
  (bind _topleft (`self.TopLeft`))
  (bind _bottomright (`self.BottomRight`))
  (bind (_navdimensions_x _navdimensions_y) (`KismetMathLibrary.BreakVector2D` (`self.NavDimensions`)))
  (bind (_boxextent_x _boxextent_y) (`KismetMathLibrary.BreakVector` (`BoxComponent.BoxExtent` (`self.Box`))))
  (bind (_relativelocation_x _relativelocation_y _relativelocation_z) (`KismetMathLibrary.BreakVector` (`SceneComponent.RelativeLocation` _bottomright)))
  (bind (_boxextent_x_2 _boxextent_y_2) (`KismetMathLibrary.BreakVector` (`BoxComponent.BoxExtent` (`self.Box`))))
  (bind (_relativelocation_x_2 _relativelocation_y_2 _relativelocation_z_2) (`KismetMathLibrary.BreakVector` (`SceneComponent.RelativeLocation` _topleft)))
  (`BoxComponent.SetBoxExtent` (`self.Box`) (`KismetMathLibrary.MakeVector` (`KismetMathLibrary.Conv_IntToDouble` (/ (* (`KismetMathLibrary.Round` (/ _navdimensions_x 100.0)) 100) 2)) (`KismetMathLibrary.Conv_IntToDouble` (/ (* (`KismetMathLibrary.Round` (/ _navdimensions_y 100.0)) 100) 2)) 50.0) true)
  (`SceneComponent.K2_SetRelativeLocation` _topleft (`KismetMathLibrary.MakeVector` (+ (- 0.0 _boxextent_x_2) 50.0) (+ (- 0.0 _boxextent_y_2) 50.0) _relativelocation_z_2) false false)
  (`SceneComponent.K2_SetRelativeLocation` _bottomright (`KismetMathLibrary.MakeVector` (- _boxextent_x 50.0) (- _boxextent_y 50.0) _relativelocation_z) false false))