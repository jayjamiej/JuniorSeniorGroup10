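; PC player controller for mouse-driven, tile-based character control, which creates the HUD and shows the cursor.
; Mouse movement traces under the cursor to send hover and click messages to actors, pausing hover updates while the scroll button is held.
; Mouse X feeds the current character's camera rotation.
; Tile moves, cancellation and character switching are delegated to the character's AI controller, with some getters left as stubs.
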(event `Init`
  (set `self.bShowMouseCursor` true)
  (bind _returnvalue (`|CreateWidget` "/Game/Blueprints/UI/TempHud.TempHud_C" self self))
  (bind _output_get (set `self.Hud` _returnvalue))
  (`UserWidget.AddToViewport` _output_get 0))

(event `self.ReceiveBeginPlay`)

(event `InputAction|ScrollPress`
  (params (Key :type "Key Structure"))
  (:`Pressed`
    (set `self.Rotating` true))
  (:`Released`
    (set `self.Rotating` false)))

(event `InputAxis|MouseX`
  (params (AxisValue :type "Float (single-precision)"))
  (bind _currentcharacter (`self.CurrentCharacter`))
  (`/Engine/EditorBlueprintResources/StandardMacros.IsValid` _currentcharacter
    (:`Is Valid`
      (bind _newrotation (`/Game/Blueprints/Characters/BP_BasePlayer_Char.RotateCam` _currentcharacter AxisValue))
      (set `self.CamRotation` _newrotation))))

(event `InputAxis|MouseMoved`
  (params (AxisValue :type "Float (single-precision)"))
  (bind (_worldlocation _worlddirection) (`self.DeprojectMousePositionToWorld`))
  (bind _selectedobject (`self.SelectedObject`))
  (if (not (`self.Rotating`))
    (`/Engine/EditorBlueprintResources/StandardMacros.IsValid` _selectedobject
      (:`Is Valid`
        (message `/Game/Blueprints/Interfaces/iMouse.MouseUnhover` _selectedobject))
      (:`Is Not Valid`
        _))
    (bind _outhit (`KismetSystemLibrary.LineTraceSingle` :`Start` _worldlocation :`End` (+ _worldlocation (* _worlddirection 10000.0)) :`TraceChannel` "TraceTypeQuery1" :`DrawTime` 1.0))
    (bind (_bblockinghit _binitialoverlap _time _distance _location _impactpoint _normal _impactnormal _physmat _hitactor) (`GameplayStatics.BreakHitResult` _outhit))
    (if _bblockinghit
      (bind _output_get (set `self.SelectedObject` _hitactor))
      (message `/Game/Blueprints/Interfaces/iMouse.MouseHover` _output_get))))

(event `InputAction|LeftClick`
  (params (Key :type "Key Structure"))
  (:`Pressed`
    (message `/Game/Blueprints/Interfaces/iMouse.MouseClick` (`self.SelectedObject`) self)))

(event `MoveCharacterTo`
  (params (Tile :type "/Game/Blueprints/Navigation/BP_NavigationTile Object Reference"))
  (bind _controller (message `/Game/Blueprints/Interfaces/iRef.getPlayerAI_Controller` (`self.GetInstigatorController` (`self.CurrentCharacter`))))
  (`/Game/Blueprints/Characters/BP_AiPlayerController_AI.MoveToTile` _controller Tile))

(event `SwitchCharacter`
  (params (Character :type "/Game/Blueprints/Characters/BP_BasePlayer_Char Object Reference"))
  (bind _output_get (set `self.CurrentCharacter` Character))
  (`/Game/Blueprints/Characters/BP_AiPlayerController_AI.SetActive` (`/Game/Blueprints/Characters/BP_BasePlayer_Char.AiController` _output_get) self))

(event `PickupObject`
  (params (Pickup :type "/Game/Blueprints/Pickups/BP_BasePickup Object Reference")))

(event `InputAction|CancelMovement`
  (params (Key :type "Key Structure"))
  (:`Pressed`
    (`/Game/Blueprints/Characters/BP_AiPlayerController_AI.CancelMovement` (`/Game/Blueprints/Characters/BP_BasePlayer_Char.AiController` (`self.CurrentCharacter`)))))

(fn `getAI`
  (returns (NewParam :type "/Game/Blueprints/Characters/BP_AiPlayerController_AI Object Reference"))
  (return (`/Game/Blueprints/Characters/BP_BasePlayer_Char.AiController` (`self.CurrentCharacter`))))

(fn `getCharacter`
  (returns (Character :type "/Game/Blueprints/Characters/BP_BasePlayer_Char Object Reference"))
  (return null))

(fn `getCurrentCharacterTile`
  (returns (Tile :type "/Game/Blueprints/Navigation/BP_NavigationTile Object Reference"))
  (return (`/Game/Blueprints/Characters/BP_BasePlayer_Char.CurrentLocation` (`self.CurrentCharacter`))))

(fn `getNavTile`
  (returns (NavTile :type "/Game/Blueprints/Navigation/BP_NavigationTile Object Reference"))
  (return null))

(fn `getPlayerAI_Controller`
  (returns (Controller :type "/Game/Blueprints/Characters/BP_AiPlayerController_AI Object Reference"))
  (return null))

(fn `getPlayerController`
  (returns (Controller :type "/Game/Blueprints/Navigation/BP_PlayerControl_PC Object Reference"))
  (return self))

(fn `getSpawnLocator`
  (returns (Locator :type "/Game/Blueprints/Navigation/BP_PlayerSpawnLocator Object Reference"))
  (return null))

(fn `UserConstructionScript`)