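; BP_TestDamage is a test actor with a sphere that subtracts incoming damage from Health and prints debug messages.
; When the damage type is BP_Burn_DT, a looping timer repeatedly subtracts half the last received damage as burn damage.
; A second timer clears the burn after a fixed duration, while a matching Delay sets the sphere's material to white.
; Nothing here handles Health reaching zero.
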(event `self.ReceiveAnyDamage`
  (params (Damage :type "Float (single-precision)") (DamageType :type "DamageType Object Reference") (InstigatedBy :type "Controller Object Reference") (DamageCauser :type "Actor Object Reference"))
  (bind _output_get (set `self.DamageAmount` Damage))
  (`KismetSystemLibrary.PrintString` "HitSphere")
  (set `self.Health` (- (`self.Health`) _output_get))
  (if (== (`GameplayStatics.GetObjectClass` DamageType) "/Game/Blueprints/DamageTypes/BP_Burn_DT.BP_Burn_DT_C")
    (bind _returnvalue (`KismetSystemLibrary.K2_SetTimerDelegate` (delegate `Burn`) 1.5 true))
    (bind _output_get_2 (set `self.BurnTimer` _returnvalue))
    (`KismetSystemLibrary.K2_SetTimerDelegate` (delegate `BurnStop`) 10.0)
    (`KismetSystemLibrary.Delay` 10.0)
    (`PrimitiveComponent.SetMaterial` (`self.Sphere`) 0 "/Game/Assets/MaterialTemp/M_White.M_White")))

(event `BurnStop`
  (`KismetSystemLibrary.K2_ClearAndInvalidateTimerHandle` (stale `self.ReceiveAnyDamage` _output_get_2)))

(event `Burn`
  (set `self.Health` (- (`self.Health`) (/ (`self.DamageAmount`) 2.0)))
  (`KismetSystemLibrary.PrintString` "Burn"))

(fn `UserConstructionScript`)