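; Game mode for a turn-based, tile-based level with three player characters sharing one player controller.
; It holds match start until BP_NavigationManager reports tiles spawned.
; The pawn spawn override possesses an ambient camera, then spawns characters on the initial spawn locator's tile and two adjacent tiles.
; After a match state change, each AI controller's turn-complete event cycles turns by ID, switching the controller to the active character.
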(event `self.ReceiveBeginPlay`
  (bind _outactors (`GameplayStatics.GetAllActorsOfClass` "/Game/Blueprints/Navigation/BP_NavigationManager.BP_NavigationManager_C"))
  (bind _output (`|GetArrayItem` _outactors))
  (add `/Game/Blueprints/Navigation/BP_NavigationManager.TilesSpawned` _output (delegate `ReadyToSpawn`))
  (`/Game/Blueprints/Navigation/BP_NavigationManager.Init` _output))

(event `ReadyToSpawn`
  (`KismetSystemLibrary.Delay` 0.5)
  (set `self.TilesSpawned` true))

(event `self.K2_OnSetMatchState`
  (params (NewState :type Name))
  (switch `name` NewState
    (:`inProgress`
      (`KismetSystemLibrary.Delay` 1.0)
      (`self.InitTurns`))))

(event `InitTurns`
  (bind _values (`BlueprintMapLibrary.Map_Values` (`self.PlayerCharacters`)))
  (for _array_element _values
    (add `/Game/Blueprints/Characters/BP_AiPlayerController_AI.onTurnComplete` (`/Game/Blueprints/Characters/BP_BasePlayer_Char.AiController` _array_element) (delegate `EndTurn`)))
  (bind _output_get (set `self.CurrentTurn` 1))
  (`self.StartTurn` _output_get))

(event `EndTurn`
  (bind _returnvalue (+ (`self.CurrentTurn`) 1))
  (bind _output_get (set `self.CurrentTurn` (select `bool` (> _returnvalue (`self.maxTurns`)) :`false` _returnvalue :`true` 1)))
  (`self.StartTurn` _output_get))

(event `StartTurn`
  (params (CharacterID :type Integer))
  (bind _output_get (set `self.ActiveCharacter` (`BlueprintMapLibrary.Map_Find` (`self.PlayerCharacters`) CharacterID)))
  (`/Game/Blueprints/Navigation/BP_PlayerControl_PC.SwitchCharacter` (`self.PlayerController`) _output_get))

(fn `FindPlayerStart`
  (params (Player :type "Controller Object Reference") (IncomingName :type String))
  (returns (ReturnValue :type "Actor Object Reference"))
  (bind _outactors (`GameplayStatics.GetAllActorsOfClass` "/Game/Blueprints/Navigation/BP_PlayerSpawnLocator.BP_PlayerSpawnLocator_C"))
  (for _array_element _outactors
    (if (`/Game/Blueprints/Navigation/BP_PlayerSpawnLocator.InitSpawn` _array_element)
      (return _array_element)))
  (return null))

(fn `ReadyToStartMatch`
  (returns (ReturnValue :type Boolean))
  (return (`self.TilesSpawned`)))

(fn `SpawnCharacterAtLocation`
  (params (SpawnTransform_Location :type "Vector Structure") (CharacterID :type Integer))
  (bind _returnvalue (`|SpawnActorFromClass` "/Game/Blueprints/Characters/BP_BasePlayer_Char.BP_BasePlayer_Char_C" (`KismetMathLibrary.MakeTransform` SpawnTransform_Location) "Undefined" "OverrideRootScale" null null))
  (`BlueprintMapLibrary.Map_Add` (`self.PlayerCharacters`) CharacterID _returnvalue)
  (`/Game/Blueprints/Characters/BP_BasePlayer_Char.Init` _returnvalue CharacterID))

(fn `SpawnDefaultPawnFor`
  (params (NewPlayer :type "Controller Object Reference") (StartSpot :type "Actor Object Reference"))
  (returns (ReturnValue :type "Pawn Object Reference"))
  (bind _controller (message `/Game/Blueprints/Interfaces/iRef.getPlayerController` NewPlayer))
  (bind _output_get (set `self.PlayerController` _controller))
  (bind _returnvalue (`|SpawnActorFromClass` "/Game/Blueprints/Characters/BP_AmbientCamera.BP_AmbientCamera_C" (`KismetMathLibrary.MakeTransform` (0.0 0.0 0.0)) "Undefined" "OverrideRootScale" null null))
  (`Controller.Possess` _output_get _returnvalue)
  (`/Game/Blueprints/Navigation/BP_PlayerControl_PC.Init` _output_get)
  (bind _locator (message `/Game/Blueprints/Interfaces/iRef.getSpawnLocator` StartSpot))
  (`|ExecutionSequence`
    (:`then_0`
      (bind _spawntile (`/Game/Blueprints/Navigation/BP_PlayerSpawnLocator.SpawnTile` _locator))
      (`self.SpawnCharacterAtLocation` (+ (`SceneComponent.K2_GetComponentLocation` (`/Game/Blueprints/Navigation/BP_NavigationTile.TileLocator` _spawntile)) (0.0 0.0 100.0)) 1))
    (:`then_1`
      (`self.SpawnCharacterAtLocation` (+ (`SceneComponent.K2_GetComponentLocation` (`/Game/Blueprints/Navigation/BP_NavigationTile.TileLocator` (`/Game/Blueprints/Navigation/BP_NavigationTile.FindAdjacentTile` _spawntile "NewEnumerator1"))) (0.0 0.0 100.0)) 2))
    (:`then_2`
      (`self.SpawnCharacterAtLocation` (+ (`SceneComponent.K2_GetComponentLocation` (`/Game/Blueprints/Navigation/BP_NavigationTile.TileLocator` (`/Game/Blueprints/Navigation/BP_NavigationTile.FindAdjacentTile` _spawntile "NewEnumerator3"))) (0.0 0.0 100.0)) 3)
      (return null))))

(fn `UserConstructionScript`)