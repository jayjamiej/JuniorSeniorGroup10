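; BP_Melee is a melee weapon whose blade moves when fired and damages actors it touches.
; Firing triggers a timeline that lerps the Box and Cube world location from StartPoint to EndPoint without sweeping.
; A DoOnce gate, reset through a short delay off the timeline update, limits retriggering.
; Any Box overlap applies fixed damage with the BP_Melee_DT damage type, with no check for an active swing.
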(event `self.Firing`
  (`self.Movemnt`))

(event `Movemnt`
  (`/Engine/EditorBlueprintResources/StandardMacros.DoOnce` false :!label _label
    (:`Completed`
      (bind (_direction _alpha) (`Timeline|MoveBlade` :!via `PlayFromStart`)
        (:`Update`
          (`SceneComponent.K2_SetWorldLocation` (`self.Box`) (`KismetMathLibrary.VLerp` (`SceneComponent.K2_GetComponentLocation` (`self.StartPoint`)) (`SceneComponent.K2_GetComponentLocation` (`self.EndPoint`)) _alpha) false false)
          (`SceneComponent.K2_SetWorldLocation` (`self.Cube`) (`KismetMathLibrary.VLerp` (`SceneComponent.K2_GetComponentLocation` (`self.StartPoint`)) (`SceneComponent.K2_GetComponentLocation` (`self.EndPoint`)) _alpha) false false)
          (`KismetSystemLibrary.Delay` 1.0)
          (goto _label :!via `Reset`))))))

(event `self.Box.OnComponentBeginOverlap`
  (params (OverlappedComponent :type "PrimitiveComponent Object Reference") (OtherActor :type "Actor Object Reference") (OtherComp :type "PrimitiveComponent Object Reference") (OtherBodyIndex :type Integer) (bFromSweep :type Boolean) (SweepResult :type "HitResult Structure (by ref)"))
  (`GameplayStatics.ApplyDamage` OtherActor 1.0 null null "/Game/Blueprints/DamageTypes/BP_Melee_DT.BP_Melee_DT_C"))

(fn `UserConstructionScript`
  (`parent.UserConstructionScript`))