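; Base player character for a tile-based game with switchable active characters, handling health, attacks, hover highlighting and a rotatable camera.
; Init spawns and possesses an AI controller and sets the WeaponMount child actor to fire, melee or heal by CharacterID.
; Capsule overlaps update the occupied nav tile, highlighting adjacent tiles while the character is active; activation also blends the view to it.
; Attack rotates the character, then messages the mounted weapon to fire.
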(event `Init`
  (params (CharacterID :type Integer))
  (bind _returnvalue (`|SpawnActorFromClass` "/Game/Blueprints/Characters/BP_AiPlayerController_AI.BP_AiPlayerController_AI_C" (`KismetMathLibrary.MakeTransform` (0.0 0.0 0.0)) "Undefined" "OverrideRootScale" null null))
  (`Controller.Possess` _returnvalue self)
  (`/Game/Blueprints/Characters/BP_AiPlayerController_AI.Init` _returnvalue self)
  (set `self.AiController` _returnvalue)
  (`ChildActorComponent.SetChildActorClass` (`self.WeaponMount`) (select `int` CharacterID :`0` null :`1` "/Game/Blueprints/Weapons/WeaponBluePrints/BP_FireWeapon.BP_FireWeapon_C" :`2` "/Game/Blueprints/Weapons/WeaponBluePrints/BP_Melee.BP_Melee_C" :`3` "/Game/Blueprints/Weapons/WeaponBluePrints/BP_Heal.BP_Heal_C" :!type "Actor Class Reference")))

(event `self.CapsuleComponent.OnComponentBeginOverlap`
  (params (OverlappedComponent :type "PrimitiveComponent Object Reference") (OtherActor :type "Actor Object Reference") (OtherComp :type "PrimitiveComponent Object Reference") (OtherBodyIndex :type Integer) (bFromSweep :type Boolean) (SweepResult :type "HitResult Structure (by ref)"))
  (`/Engine/EditorBlueprintResources/StandardMacros.DoOnce` false :!label _label
    (:`Completed`
      (bind _navtile (message `/Game/Blueprints/Interfaces/iRef.getNavTile` OtherActor))
      (`/Engine/EditorBlueprintResources/StandardMacros.IsValid` _navtile
        (:`Is Valid`
          (`/Engine/EditorBlueprintResources/StandardMacros.IsValid` (`self.CurrentLocation`)
            (:`Is Valid`
              (`self.HighlightDirections` false)
              (`/Game/Blueprints/Navigation/BP_NavigationTile.SetOccupied` (`self.CurrentLocation`) false))
            (:`Is Not Valid`
              _))
          (bind _output_get (set `self.CurrentLocation` _navtile))
          (`/Game/Blueprints/Navigation/BP_NavigationTile.SetOccupied` _output_get true)
          (if (`self.IsActiveCharacter`)
            (`self.HighlightDirections` true))
          (`KismetSystemLibrary.Delay` 0.5)
          (goto _label :!via `Reset`))
        (:`Is Not Valid`
          (goto _label :!via `Reset`))))))

(event `ActivateCharacter`
  (params (PlayerController :type "/Game/Blueprints/Navigation/BP_PlayerControl_PC Object Reference"))
  (set `self.IsActiveCharacter` true)
  (`PlayerController.SetViewTargetWithBlend` PlayerController self 1.0 "VTBlend_Linear" 0.0 false)
  (`self.HighlightDirections` true))

(event `DeactivateCharacter`
  (set `self.IsActiveCharacter` false)
  (`self.HighlightDirections` false))

(event `/Game/Blueprints/Weapons/iWeapons.Heal`
  ;[1 1 1] Weapon Heal
  (if (>= (`self.Health`) (`self.MaxHealth`))
    (set `self.Health` (`self.MaxHealth`))
    (else
      (set `self.Health` (+ (`self.Health`) (`self.HealAmount`))))))

(event `Attack`
  (params (AttackRotation :type "Rotator Structure"))
  (bind _returnvalue (`self.K2_SetActorRotation` AttackRotation))
  (if _returnvalue
    (message `/Game/Blueprints/Weapons/iWeapons.Fire` (`ChildActorComponent.ChildActor` (`self.WeaponMount`)))))

(event `/Game/Blueprints/Interfaces/iMouse.MouseClick`
  (params (Controller :type "/Game/Blueprints/Navigation/BP_PlayerControl_PC Object Reference")))

(event `Key|F`
  (params (Key :type "Key Structure"))
  ;[0.07292 0.07292 1] Random Damage For Debug
  (:`Pressed`
    (set `self.Health` (- (`self.Health`) 25.0))))

(event `/Game/Blueprints/Interfaces/iMouse.MouseHover`
  (bind _mesh (`self.Mesh`))
  (`PrimitiveComponent.SetMaterial` _mesh 0 "/Game/Blueprints/Characters/M_CharHighlight_Temp.M_CharHighlight_Temp")
  (`PrimitiveComponent.SetMaterial` _mesh 1 "/Game/Blueprints/Characters/MI_CharChestHighlight_Temp.MI_CharChestHighlight_Temp"))

(event `/Game/Blueprints/Interfaces/iMouse.MouseUnhover`
  (bind _mesh (`self.Mesh`))
  (`PrimitiveComponent.SetMaterial` _mesh 0 "/Game/Assets/AnimTemp/AnimStarterPack/UE4_Mannequin/Materials/M_UE4Man_Body.M_UE4Man_Body")
  (`PrimitiveComponent.SetMaterial` _mesh 1 "/Game/Assets/AnimTemp/AnimStarterPack/UE4_Mannequin/Materials/M_UE4Man_ChestLogo.M_UE4Man_ChestLogo"))

(event `self.ReceiveAnyDamage`
  (params (Damage :type "Float (single-precision)") (DamageType :type "DamageType Object Reference") (InstigatedBy :type "Controller Object Reference") (DamageCauser :type "Actor Object Reference"))
  (set `self.Health` (- (`self.Health`) Damage)))

(fn `getCharacter`
  (returns (Character :type "/Game/Blueprints/Characters/BP_BasePlayer_Char Object Reference"))
  (return self))

(fn `getNavTile`
  (returns (NavTile :type "/Game/Blueprints/Navigation/BP_NavigationTile Object Reference"))
  (return null))

(fn `getPlayerAI_Controller`
  (returns (Controller :type "/Game/Blueprints/Characters/BP_AiPlayerController_AI Object Reference"))
  (return null))

(fn `getPlayerController`
  (returns (Controller :type "/Game/Blueprints/Navigation/BP_PlayerControl_PC Object Reference"))
  (return null))

(fn `getSpawnLocator`
  (returns (Locator :type "/Game/Blueprints/Navigation/BP_PlayerSpawnLocator Object Reference"))
  (return null))

(fn `HighlightDirections`
  (params (Active :type Boolean))
  (bind _values (`BlueprintMapLibrary.Map_Values` (`/Game/Blueprints/Navigation/BP_NavigationTile.AdjacentTiles` (`self.CurrentLocation`))))
  (for _array_element _values
    (`/Game/Blueprints/Navigation/BP_NavigationTile.Directions` _array_element Active)))

(fn `RotateCam`
  (params (AxisVal :type "Float (double-precision)"))
  (returns (NewRotation :type "Rotator Structure"))
  (`SceneComponent.K2_AddRelativeRotation` (`self.SpringArm`) (`KismetMathLibrary.MakeRotator` 0.0 0.0 (* AxisVal 2.0)) false false)
  (return (`SceneComponent.K2_GetComponentRotation` (`self.SpringArm`))))

(fn `SwitchToCam`
  (params (Controller :type "/Game/Blueprints/Navigation/BP_PlayerControl_PC Object Reference"))
  (`PlayerController.SetViewTargetWithBlend` Controller self 1.0 "VTBlend_Linear" 0.0 false))

(fn `UserConstructionScript`)