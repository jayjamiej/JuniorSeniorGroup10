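; BP_Weapon is a beam weapon that deals repeated damage to whatever lies in front of it while firing.
; FireWeapon activates the beam particle and starts a looping timer, and StopFire deactivates the beam and clears the timer.
; On each tick of the timer, a short-range sphere trace runs forward from an Arrow component and applies DamageAmount to the actor it hits.
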(event `/Game/iObjectInteractions.StopFire`
  ;[1 1 1] Weapon Firing+LineTrace
  (`ActorComponent.Deactivate` (`self.Beam_PAR`))
  (`KismetSystemLibrary.K2_ClearAndInvalidateTimerHandle` (stale `/Game/iObjectInteractions.FireWeapon` _returnvalue)))

(event `/Game/iObjectInteractions.FireWeapon`
  ;[1 1 1] Weapon Firing+LineTrace
  (`ActorComponent.Activate` (`self.Beam_PAR`) false)
  (bind _returnvalue (`KismetSystemLibrary.K2_SetTimerDelegate` (delegate `Shooting`) 0.25 true)))

(event `Shooting`
  (bind _arrow (`self.Arrow`))
  (bind _returnvalue (`SceneComponent.K2_GetComponentLocation` _arrow))
  ;[1 1 1] Weapon Firing+LineTrace
  (bind _outhit (`KismetSystemLibrary.SphereTraceSingle` :`Start` _returnvalue :`End` (+ _returnvalue (* (`SceneComponent.GetForwardVector` _arrow) 500.0)) :`Radius` 35.0 :`TraceChannel` "TraceTypeQuery1" :`DrawTime` 1.0))
  (`GameplayStatics.ApplyDamage` (`.HitActor` (`GameplayStatics.BreakHitResult` _outhit)) (`self.damageAmount`)))

(fn `UserConstructionScript`)