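; BP_RoomBounds marks a room volume for ghost AI, with its box sized from VolumeExtents on construction.
; An overlapping AI-controlled actor gets this room written to its blackboard's Room key, plus a debug print.
; GetRandomFurniture picks from the room's Furniture list, recursing to avoid possessed pieces when requested.
; Its check and return roll separate random indices, so a possessed piece can still be returned.
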(event `self.Volume.OnComponentBeginOverlap`
  (params (OverlappedComponent :type "PrimitiveComponent Object Reference") (OtherActor :type "Actor Object Reference") (OtherComp :type "PrimitiveComponent Object Reference") (OtherBodyIndex :type Integer) (bFromSweep :type Boolean) (SweepResult :type "HitResult Structure (by ref)"))
  (bind _returnvalue (`AIBlueprintHelperLibrary.GetAIController` OtherActor))
  (`/Engine/EditorBlueprintResources/StandardMacros.IsValid` _returnvalue
    (:`Is Valid`
      (`BlackboardComponent.SetValueAsObject` (`AIBlueprintHelperLibrary.GetBlackboard` _returnvalue) "Room" self)
      (`KismetSystemLibrary.PrintString` "Ghost Detected"))))

(fn `GetRandomFurniture`
  (params (NotPossessed :type Boolean))
  (returns (Furniture :type "/Game/Blueprint/BP_Furniture Object Reference"))
  (bind _furniture (`self.Furniture`))
  (bind _output (`|GetArrayItem` _furniture (`KismetMathLibrary.RandomIntegerInRange` 0 (`KismetArrayLibrary.Array_LastIndex` _furniture))))
  (if NotPossessed
    (if (`/Game/Blueprint/BP_Furniture.IsPossessed` _output)
      (bind _furniture_2 (`self.GetRandomFurniture` true))
      (return _furniture_2)
      (else
        _)))
  (return _output))

(fn `UserConstructionScript`
  (`BoxComponent.SetBoxExtent` (`self.Volume`) (`self.VolumeExtents`) true))