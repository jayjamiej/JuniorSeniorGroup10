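; Manager for a ghost AI path that holds an array of indexed point actors and serves waypoints on request.
; FindNextPoint steps the current index forward or backward, recursing at the path's end to either loop to the start or bounce into reverse.
; Lookup functions scan the array for a point by its Index value or for the one closest to a world location.
; All event graph events are empty, so the logic lives entirely in these functions.
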(fn `FindNextPoint`
  (returns (Point :type "/Game/Blueprint/AI/Path/BP_EnemyPathPoint Object Reference"))
  (bind _pointindex (`self.PointIndex`))
  (if (== (`self.PointIndex`) (select `bool` (`self.IsReversing`) :`false` (`KismetArrayLibrary.Array_LastIndex` (`self.Paths`))))
    (switch `/Game/Blueprint/AI/Path/ePathEndHandling` (`self.EndHandling`)
      (:`NewEnumerator0`
        (set `self.PointIndex` -1))
      (:`NewEnumerator1`
        (set `self.IsReversing` (not (`self.IsReversing`)))))
    (bind _point (`self.FindNextPoint`))
    (return _point)
    (else
      (set `self.PointIndex` (select `bool` (`self.IsReversing`) :`false` (+ _pointindex 1) :`true` (- _pointindex 1)))
      (for _array_element (`self.Paths`)
        (if (== (`/Game/Blueprint/AI/Path/BP_EnemyPathPoint.Index` _array_element) (`self.PointIndex`))
          (return _array_element))))))

(fn `GetClosestPoint`
  (params (WorldLocation :type "Vector Structure"))
  (returns (Point :type "/Game/Blueprint/AI/Path/BP_EnemyPathPoint Object Reference"))
  (locals (ClosestDistance :type "Float (double-precision)" :default 500000.0) (Closest :type "/Game/Blueprint/AI/Path/BP_EnemyPathPoint Object Reference"))
  (for _array_element (`self.Paths`)
    (bind _returnvalue (`KismetMathLibrary.Vector_Distance` (`self.K2_GetActorLocation` _array_element) WorldLocation))
    (if (< _returnvalue (`local.ClosestDistance`))
      (set `local.ClosestDistance` _returnvalue)
      (set `local.Closest` _array_element)))
  (return (`local.Closest`)))

(fn `GetPointAtIndex`
  (params (Index :type Integer))
  (returns (Point :type "/Game/Blueprint/AI/Path/BP_EnemyPathPoint Object Reference"))
  (for _array_element (`self.Paths`)
    (if (== (`/Game/Blueprint/AI/Path/BP_EnemyPathPoint.Index` _array_element) Index)
      (return _array_element)))
  (return null))

(fn `UserConstructionScript`)