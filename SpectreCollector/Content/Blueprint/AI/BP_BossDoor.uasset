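; Boss door that unlocks once every ghost in its MiniBosses list is dusted.
; Each OnDusted event raises a count that sets the meter material's Percent and drives a timeline scaling the fill on Z.
; When the fill finishes at full, BP_GhostPlayer entering the sphere swings both doors open once via a timeline.
; GetTargetWorldLocation returns a point above the actor.
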(event `self.ReceiveBeginPlay`
  ;[1 1 1] Init
  (bind _returnvalue (`PrimitiveComponent.CreateDynamicMaterialInstance` (`self.Cylinder`) 0 "/Game/Blueprint/AI/GhostMeter.GhostMeter" "None"))
  (set `self.MeterMaterial` _returnvalue)
  (for _array_element (`self.MiniBosses`)
    (add `/Game/Blueprint/AI/Pawns/BP_BaseGhost.OnDusted` _array_element (delegate `GhostDowned`))))

(event `GhostDowned`
  (params (GhostDusted :type "/Game/Blueprint/AI/Pawns/BP_BaseGhost Object Reference"))
  (bind _percent_temp (`self.Percent_Temp`))
  (bind (_relativescale3d_x _relativescale3d_y _relativescale3d_z) (`KismetMathLibrary.BreakVector` (`SceneComponent.RelativeScale3D` (`self.Scene`))))
  ;[1 1 1] UpdatingMeter
  (bind _result (`/Engine/EditorBlueprintResources/StandardMacros.IncrementInt` (`self.DownedGhosts`))
    (:`  `
      (bind _returnvalue (/ (`KismetMathLibrary.Conv_IntToDouble` _result) (`KismetMathLibrary.Conv_IntToDouble` (`KismetArrayLibrary.Array_Length` (`self.MiniBosses`)))))
      (`MaterialInstanceDynamic.SetScalarParameterValue` (`self.MeterMaterial`) "Percent" _returnvalue)
      (set `self.Percent_Temp` _returnvalue)
      (set `self.PercentCurrent_Temp` _relativescale3d_z)
      (bind (_direction _alpha) (`Timeline|MeterFill` :!via `PlayFromStart`)
        (:`Update`
          (`SceneComponent.SetRelativeScale3D` (`self.Scene`) (`KismetMathLibrary.MakeVector` 1.0 1.0 (`KismetMathLibrary.Lerp` (`self.PercentCurrent_Temp`) _percent_temp _alpha))))
        (:`Finished`
          ;[1 1 1] Unlock door if equal to 1
          (set `self.CanOpenDoor` (== _percent_temp 1.0)))))))

(event `self.Sphere.OnComponentBeginOverlap`
  (params (OverlappedComponent :type "PrimitiveComponent Object Reference") (OtherActor :type "Actor Object Reference") (OtherComp :type "PrimitiveComponent Object Reference") (OtherBodyIndex :type Integer) (bFromSweep :type Boolean) (SweepResult :type "HitResult Structure (by ref)"))
  ;[1 1 1] Opens door when player is near
  (if (== (`GameplayStatics.GetObjectClass` OtherActor) "/Game/Blueprint/BP_GhostPlayer.BP_GhostPlayer_C")
    (if (`self.CanOpenDoor`)
      (`/Engine/EditorBlueprintResources/StandardMacros.DoOnce` false
        (:`Completed`
          (bind (_direction _alpha) (`Timeline|DoorOpen` :!via `PlayFromStart`)
            (:`Update`
              (bind _returnvalue (`KismetMathLibrary.Lerp` 0.0 65.0 _alpha))
              (`SceneComponent.K2_SetRelativeRotation` (`self.DoorLeft`) (`KismetMathLibrary.MakeRotator` 0.0 0.0 _returnvalue) false false)
              (`SceneComponent.K2_SetRelativeRotation` (`self.DoorRight`) (`KismetMathLibrary.MakeRotator` 0.0 0.0 (- -10.0 _returnvalue)) false false))))))))

(fn `GetTargetWorldLocation`
  (returns (Target :type "Vector Structure"))
  (return (+ (`self.K2_GetActorLocation`) (0.0 0.0 150.0))))

(fn `UserConstructionScript`)