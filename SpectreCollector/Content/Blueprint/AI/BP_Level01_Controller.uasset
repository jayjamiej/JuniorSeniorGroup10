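; BP_Level01_Controller is an AI controller, named for Level 01, that starts its behavior tree on BeginPlay.
; It then seeds the IsHiding blackboard key from the InstantHide variable, so the tree knows whether the AI begins hidden.
; Of its getter functions, only GetEnemyController returns a value (itself); the furniture, player character and player controller getters are empty stubs.
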(event `self.ReceiveBeginPlay`
  (`self.RunBehaviorTree` (`self.BehaviourTree`))
  (`BlackboardComponent.SetValueAsBool` (`AIBlueprintHelperLibrary.GetBlackboard` null) "IsHiding" (`self.InstantHide`)))

(fn `getEnemyController`
  (returns (Controller :type "/Game/Blueprint/AI/BP_Level01_Controller Object Reference"))
  (return self))

(fn `getFurniture`
  (returns (Furniture :type "/Game/Blueprint/BP_Furniture Object Reference"))
  (return null))

(fn `getPlayerCharacter`
  (returns (Character :type "/Game/Blueprint/BP_GhostPlayer Object Reference"))
  (return null))

(fn `getPlayerController`
  (returns (Controller :type "/Game/Blueprint/BP_PlayerController Object Reference"))
  (return null))

(fn `UserConstructionScript`)