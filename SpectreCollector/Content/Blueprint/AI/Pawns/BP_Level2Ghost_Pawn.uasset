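; BP_Level2Ghost_Pawn is an AI ghost enemy pawn for level 2 that goes into hiding when it takes damage or attacks.
; Its damage behaviour lowers walk speed and starts a timer that restores it, with repeated hits restarting the timer.
; Both damage and attack, which also calls the parent attack, set the IsHiding blackboard key on its AI controller.
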(event `self.DamagedBehaviour`
  (if (`KismetSystemLibrary.K2_IsValidTimerHandle` (`self.SlowCooldown`))
    (`KismetSystemLibrary.K2_ClearAndInvalidateTimerHandle` (`self.SlowCooldown`)))
  (set `CharacterMovementComponent.MaxWalkSpeed` 100.0 (`self.CharacterMovement`))
  (bind _returnvalue (`KismetSystemLibrary.K2_SetTimerDelegate` (delegate `ResetSpeed`) 5.0))
  (set `self.SlowCooldown` _returnvalue)
  (`BlackboardComponent.SetValueAsBool` (`AIBlueprintHelperLibrary.GetBlackboard` (`AIBlueprintHelperLibrary.GetAIController` self)) "IsHiding" true))

(event `ResetSpeed`
  (set `CharacterMovementComponent.MaxWalkSpeed` 300.0 (`self.CharacterMovement`)))

(event `self.Attack`
  (params (Forced :type Boolean))
  (`parent.Attack` false)
  (`BlackboardComponent.SetValueAsBool` (`AIBlueprintHelperLibrary.GetBlackboard` (`AIBlueprintHelperLibrary.GetAIController` self)) "IsHiding" true))

(fn `UserConstructionScript`
  (`parent.UserConstructionScript`))