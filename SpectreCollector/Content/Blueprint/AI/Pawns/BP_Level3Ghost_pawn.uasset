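; Level 3 ghost enemy pawn that follows a path and fires projectiles.
; On BeginPlay it writes the location of the PathManager's first point to its AI controller's blackboard as PathLocation.
; A looping timer drives the Attack event, which spawns an enemy projectile at the Arrow1 component's transform with the ghost as owner.
; GetEnemyPathManager exposes the path manager.
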(event `self.ReceiveBeginPlay`
  (`parent.ReceiveBeginPlay`)
  (bind _point (`/Game/Blueprint/AI/Path/BP_GhostPath_Manager.GetPointAtIndex` (`self.PathManager`) 0))
  (`BlackboardComponent.SetValueAsVector` (`AIBlueprintHelperLibrary.GetBlackboard` (`AIBlueprintHelperLibrary.GetAIController` self)) "PathLocation" (`self.K2_GetActorLocation` _point))
  (`KismetSystemLibrary.K2_SetTimerDelegate` (delegate `self.Attack`) 2.0 true))

(event `self.Attack`
  (`|SpawnActorFromClass` "/Game/Blueprint/AI/BP_EnemyProjectile.BP_EnemyProjectile_C" (`SceneComponent.K2_GetComponentToWorld` (`self.Arrow1`)) "Undefined" "OverrideRootScale" self null))

(fn `GetEnemyPathManager`
  (returns (Manager :type "/Game/Blueprint/AI/Path/BP_GhostPath_Manager Object Reference"))
  (return (`self.PathManager`)))

(fn `UserConstructionScript`
  (`parent.UserConstructionScript`))