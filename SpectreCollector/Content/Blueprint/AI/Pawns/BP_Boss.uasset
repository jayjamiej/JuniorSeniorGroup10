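; BP_Boss is an AI boss pawn that damages what it hits and fires projectiles.
; On BeginPlay it seeds the blackboard's PathLocation with the first point from its PathManager, which it also exposes through a getter.
; Capsule hits apply damage and send a knockback message along the impact normal.
; Attack spawns one BP_BossProjectile from an arrow component, or one from each of three arrows when Forced.
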(event `self.ReceiveBeginPlay`
  (`parent.ReceiveBeginPlay`)
  (bind _point (`/Game/Blueprint/AI/Path/BP_GhostPath_Manager.GetPointAtIndex` (`self.PathManager`) 0))
  (`BlackboardComponent.SetValueAsVector` (`AIBlueprintHelperLibrary.GetBlackboard` (`AIBlueprintHelperLibrary.GetAIController` self)) "PathLocation" (`self.K2_GetActorLocation` _point)))

(event `self.Capsule.OnComponentHit`
  (params (HitComponent :type "PrimitiveComponent Object Reference") (OtherActor :type "Actor Object Reference") (OtherComp :type "PrimitiveComponent Object Reference") (NormalImpulse :type "Vector Structure") (Hit :type "HitResult Structure (by ref)"))
  (message `/Game/Blueprint/iPlayer.AddKnockback` OtherActor (* (`.ImpactNormal` (`GameplayStatics.BreakHitResult` Hit)) -7500.0))
  (`GameplayStatics.ApplyDamage` OtherActor 50.0))

(event `self.Attack`
  (params (Forced :type Boolean))
  (bind (_returnvalue_location _returnvalue_rotation) (`KismetMathLibrary.BreakTransform` (`SceneComponent.K2_GetComponentToWorld` (`self.Arrow1`))))
  (if (not Forced)
    (`|SpawnActorFromClass` "/Game/Blueprint/AI/BP_BossProjectile.BP_BossProjectile_C" (`KismetMathLibrary.MakeTransform` _returnvalue_location _returnvalue_rotation) "Undefined" "OverrideRootScale" null null)
    (else
      (for _array_element (`|MakeArray` (`self.Arrow1`) (`self.Arrow2`) (`self.Arrow3`))
        (bind (_returnvalue_location_2 _returnvalue_rotation_2) (`KismetMathLibrary.BreakTransform` (`SceneComponent.K2_GetComponentToWorld` _array_element)))
        (`|SpawnActorFromClass` "/Game/Blueprint/AI/BP_BossProjectile.BP_BossProjectile_C" (`KismetMathLibrary.MakeTransform` _returnvalue_location_2 _returnvalue_rotation_2) "Undefined" "OverrideRootScale" null null)))))

(fn `GetEnemyPathManager`
  (returns (Manager :type "/Game/Blueprint/AI/Path/BP_GhostPath_Manager Object Reference"))
  (return (`self.PathManager`)))

(fn `UserConstructionScript`
  (`parent.UserConstructionScript`))