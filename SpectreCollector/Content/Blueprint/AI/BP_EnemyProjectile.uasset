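; Enemy projectile actor that deals BP_GhostDamage to whatever it hits, then breaks apart.
; It ignores its owner while moving, and its mesh and uniform scale are set in the construction script and spun every tick.
; A hit or any incoming damage calls a shared Destroy function that plays a poof particle and break sound before removing the actor.
; GetTargetWorldLocation exposes the mesh's world position.
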(event `self.ReceiveBeginPlay`
  (`PrimitiveComponent.IgnoreActorWhenMoving` (`self.RootCollision`) (`self.GetOwner`) true))

(event `self.RootCollision.OnComponentHit`
  (params (HitComponent :type "PrimitiveComponent Object Reference") (OtherActor :type "Actor Object Reference") (OtherComp :type "PrimitiveComponent Object Reference") (NormalImpulse :type "Vector Structure") (Hit :type "HitResult Structure (by ref)"))
  (`GameplayStatics.ApplyDamage` OtherActor (`self.Damage`) null (`self.GetOwner`) "/Game/Blueprint/BP_GhostDamage.BP_GhostDamage_C")
  (`self.Destroy` (`.Location` (`GameplayStatics.BreakHitResult` Hit)) OtherActor))

(event `self.ReceiveTick`
  (params (DeltaSeconds :type "Float (single-precision)"))
  (`SceneComponent.K2_AddRelativeRotation` (`self.ProjectileMesh`) (struct :`Pitch` -1.0 :`Yaw` 1.0 :`Roll` -1.0) false false))

(event `self.ReceiveAnyDamage`
  (params (Damage :type "Float (single-precision)") (DamageType :type "DamageType Object Reference") (InstigatedBy :type "Controller Object Reference") (DamageCauser :type "Actor Object Reference"))
  (`self.Destroy` (`self.K2_GetActorLocation`)))

(fn `Destroy`
  (params (Location :type "Vector Structure") (HitActor :type "Actor Object Reference"))
  (`GameplayStatics.SpawnEmitterAtLocation` "/Game/Particles/PS_ProjectilePoof.PS_ProjectilePoof" Location)
  (`GameplayStatics.PlaySoundAtLocation` (`self.BreakSound`) Location (struct) 1.0 1.0 0.0 null null null)
  (`self.K2_DestroyActor`))

(fn `GetTargetWorldLocation`
  (returns (Target :type "Vector Structure"))
  (return (`SceneComponent.K2_GetComponentLocation` (`self.ProjectileMesh`))))

(fn `UserConstructionScript`
  (`StaticMeshComponent.SetStaticMesh` (`self.ProjectileMesh`) (`self.Mesh`))
  (`SceneComponent.SetRelativeScale3D` (`self.ProjectileMesh`) (`KismetMathLibrary.Conv_DoubleToVector` (`self.meshScale`))))