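; AI controller for Level01 that runs a behavior tree and seeds its blackboard at BeginPlay.
; It sets IsHiding from InstantHide, then after a short delay sets MoveToLocation to a random reachable point around the controlled pawn.
; The furniture, player character and player controller getters are empty stubs.
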(event `self.ReceiveBeginPlay`
  (bind _returnvalue (`AIBlueprintHelperLibrary.GetBlackboard` null))
  (bind _returnvalue_2 (`self.RunBehaviorTree` (`self.BehaviourTree`)))
  (`KismetSystemLibrary.PrintString` (`KismetStringLibrary.Conv_BoolToString` _returnvalue_2))
  (`BlackboardComponent.SetValueAsBool` _returnvalue "IsHiding" (`self.InstantHide`))
  (`KismetSystemLibrary.Delay` 0.2)
  (`BlackboardComponent.SetValueAsVector` _returnvalue "MoveToLocation" (`NavigationSystemV1.K2_GetRandomReachablePointInRadius` (`self.K2_GetActorLocation` (`self.K2_GetPawn`)) 1000.0 null null)))

(fn `getFurniture`
  (returns (Furniture :type "/Game/Jamie_D/BP_Furniture Object Reference"))
  (return null))

(fn `getPlayerCharacter`
  (returns (Character :type "/Game/Blueprint/BP_GhostPlayer Object Reference"))
  (return null))

(fn `getPlayerController`
  (returns (Controller :type "/Game/Blueprint/BP_PlayerController Object Reference"))
  (return null))

(fn `UserConstructionScript`)