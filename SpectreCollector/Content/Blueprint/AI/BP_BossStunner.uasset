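; Boss stunner actor that, when damaged, has a chance to set the IsStunned blackboard key on the referenced Boss's AI controller.
; A DoOnce gates hits, and a separately evaluated random roll decides whether PSMusic switches off for a delay before reactivating and reopening the gate, or reopens it immediately.
; IsStunned is only rewritten on the next accepted hit, with no timed clear.
; The construction script applies the configurable Cube mesh, whose location is exposed as the target location.
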(event `self.ReceiveAnyDamage`
  (params (Damage :type "Float (single-precision)") (DamageType :type "DamageType Object Reference") (InstigatedBy :type "Controller Object Reference") (DamageCauser :type "Actor Object Reference"))
  (bind _returnvalue (`KismetMathLibrary.RandomBoolWithWeight` 0.2))
  (`/Engine/EditorBlueprintResources/StandardMacros.DoOnce` false :!label _label
    (:`Completed`
      (`BlackboardComponent.SetValueAsBool` (`AIBlueprintHelperLibrary.GetBlackboard` (`AIBlueprintHelperLibrary.GetAIController` (`self.Boss`))) "IsStunned" _returnvalue)
      (if _returnvalue
        (`ActorComponent.Deactivate` (`self.PS_Music`))
        (`KismetSystemLibrary.Delay` 5.0)
        (`ActorComponent.Activate` (`self.PS_Music`) false)
        (goto _label :!via `Reset`)
        (else
          (goto _label :!via `Reset`))))))

(fn `GetTargetWorldLocation`
  (returns (Target :type "Vector Structure"))
  (return (`SceneComponent.K2_GetComponentLocation` (`self.Cube`))))

(fn `UserConstructionScript`
  (`StaticMeshComponent.SetStaticMesh` (`self.Cube`) (`self.Mesh`)))