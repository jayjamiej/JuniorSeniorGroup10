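; BP_Level3Respawner respawns a Level 3 ghost at its own transform after the bound Boss fires its OnDusted event.
; On BeginPlay it caches the referenced Level3Ghost's path manager, icon, mesh, animation, name and projectile settings.
; Two seconds after the dusted event, it spawns a new BP_Level3Ghost_pawn configured with those cached values and prints a debug message.
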(event `self.ReceiveBeginPlay`
  (bind _level3ghost (`self.Level3Ghost`))
  (add `/Game/Blueprint/AI/Pawns/BP_BaseGhost.OnDusted` (`self.Boss`) (delegate `GhostDown`))
  (set `self.GhostPathManager` (`/Game/Blueprint/AI/Pawns/BP_Level3Ghost_pawn.PathManager` _level3ghost))
  (set `self.GhostIcon` (`/Game/Blueprint/AI/Pawns/BP_Level3Ghost_pawn.GhostIcon` _level3ghost))
  (set `self.GhostMesh` (`/Game/Blueprint/AI/Pawns/BP_Level3Ghost_pawn.GhostMesh` _level3ghost))
  (set `self.Anim` (`/Game/Blueprint/AI/Pawns/BP_Level3Ghost_pawn.GhostAnim` _level3ghost))
  (set `self.GhostName` (`/Game/Blueprint/AI/Pawns/BP_Level3Ghost_pawn.GhostName` _level3ghost))
  (set `self.ProjectileMesh` (`/Game/Blueprint/AI/Pawns/BP_Level3Ghost_pawn.ProjectileMesh` _level3ghost))
  (set `self.ProjectileScale` (`/Game/Blueprint/AI/Pawns/BP_Level3Ghost_pawn.ProjectileScale` _level3ghost))
  (set `self.ProjectileSound` (`/Game/Blueprint/AI/Pawns/BP_Level3Ghost_pawn.ProjectileSound` _level3ghost)))

(event `GhostDown`
  (params (GhostDusted :type "/Game/Blueprint/AI/Pawns/BP_BaseGhost Object Reference"))
  (`KismetSystemLibrary.Delay` 2.0)
  (`|SpawnActorFromClass` "/Game/Blueprint/AI/Pawns/BP_Level3Ghost_pawn.BP_Level3Ghost_pawn_C" (`self.GetTransform`) "Undefined" "OverrideRootScale" null (`self.GhostPathManager`) (`self.GhostIcon`) (`self.GhostMesh`) (`self.GhostName`) (`self.Anim`) (`self.ProjectileMesh`) (`self.ProjectileScale`) (`self.ProjectileSound`) 250.0 null null)
  (`KismetSystemLibrary.PrintString` "Respawned"))

(fn `UserConstructionScript`)