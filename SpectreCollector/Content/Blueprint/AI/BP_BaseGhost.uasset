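; Base ghost enemy character that attacks by hand, can possess furniture and drops a dust pickup on death.
; Taking damage sets walk speed, plays a head-bob timeline and lowers Health, destroying the actor at zero.
; StunAttack is gated by a DoOnce reset when its hand-swing timeline ends, enabling hand collision only during the swing to apply ghost damage on overlap.
; Getter functions return self for the enemy and are otherwise empty.
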(event `self.ReceiveBeginPlay`
  (`parent.ReceiveBeginPlay`)
  (`PrimitiveComponent.SetCollisionEnabled` (`self.HandCol`) "NoCollision"))

(event `self.ReceiveAnyDamage`
  (params (Damage :type "Float (single-precision)") (DamageType :type "DamageType Object Reference") (InstigatedBy :type "Controller Object Reference") (DamageCauser :type "Actor Object Reference"))
  (set `CharacterMovementComponent.MaxWalkSpeed` 400.0 (`self.CharacterMovement`))
  (`self.HitAnim`)
  (`self.Damage` Damage)
  (if (<= (`self.Health`) 0.0)
    (`|SpawnActorFromClass` "/Game/Blueprint/BP_DustPickup.BP_DustPickup_C" (`SceneComponent.K2_GetComponentToWorld` (`self.DustSpawn`)) "AlwaysSpawn" "OverrideRootScale" null 50 null)
    (`self.Death`)))

(event `HitAnim`
  (bind (_direction _alpha) (`Timeline|HeadUp`)
    (:`Update`
      (`SceneComponent.K2_SetRelativeLocation` (`self.Head`) (`KismetMathLibrary.VLerp` (0.0 15.0 135.0) (0.0 15.0 175.0) _alpha) false false))))

(event `StunAttack`
  (`/Engine/EditorBlueprintResources/StandardMacros.DoOnce` false :!label _label
    (:`Completed`
      (`PrimitiveComponent.SetCollisionEnabled` (`self.HandCol`) "QueryOnly")
      (bind (_direction _alpha) (`Timeline|Attack` :!via `PlayFromStart`)
        (:`Update`
          (`SceneComponent.K2_SetRelativeLocation` (`self.RightHand`) (`KismetMathLibrary.VLerp` (-50.0 40.0 15.0) (-50.0 120.0 15.0) _alpha) false false))
        (:`Finished`
          (`PrimitiveComponent.SetCollisionEnabled` (`self.HandCol`) "NoCollision")
          (`self.ResetStun`))))))

(event `ResetStun`
  (goto _label :!via `Reset`))

(event `self.HandCol.OnComponentBeginOverlap`
  (params (OverlappedComponent :type "PrimitiveComponent Object Reference") (OtherActor :type "Actor Object Reference") (OtherComp :type "PrimitiveComponent Object Reference") (OtherBodyIndex :type Integer) (bFromSweep :type Boolean) (SweepResult :type "HitResult Structure (by ref)"))
  (`GameplayStatics.ApplyDamage` OtherActor 0.25 null null "/Game/Blueprint/BP_GhostDamage.BP_GhostDamage_C"))

(event `PossessFurniture`
  (params (Furniture :type "/Game/Blueprint/BP_Furniture Object Reference"))
  (`/Game/Blueprint/BP_Furniture.Possess` Furniture self))

(fn `Damage`
  (params (Damage :type "Float (double-precision)"))
  (set `self.Health` (- (`self.Health`) Damage)))

(fn `Death`
  (`self.K2_DestroyActor`))

(fn `getEnemy`
  (returns (Ghost :type "/Game/Blueprint/AI/BP_BaseGhost Object Reference"))
  (return self))

(fn `getEnemyController`
  (returns (Controller :type "/Game/Blueprint/AI/BP_Level01_Controller Object Reference"))
  (return null))

(fn `getFurniture`
  (returns (Furniture :type "/Game/Blueprint/BP_Furniture Object Reference"))
  (return null))

(fn `getPlayerCharacter`
  (returns (Character :type "/Game/Blueprint/BP_GhostPlayer Object Reference"))
  (return null))

(fn `getPlayerController`
  (returns (Controller :type "/Game/Blueprint/BP_PlayerController Object Reference"))
  (return null))

(fn `UserConstructionScript`
  (`parent.UserConstructionScript`))