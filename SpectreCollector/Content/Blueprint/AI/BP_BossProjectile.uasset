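; Boss projectile Blueprint that can spawn a fodder ghost enemy where it hits.
; It extends a parent projectile by overriding the Destroy event, which receives the impact location and hit actor.
; If the hit actor is not a ghost player, it spawns a BP_FodderGhost with preset health there and sets an ignore-when-moving flag through the root collision.
; The parent's Destroy logic runs afterward.
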(event `self.Destroy`
  (params (Location :type "Vector Structure") (HitActor :type "Actor Object Reference"))
  (if (not (`KismetMathLibrary.ClassIsChildOf` (`GameplayStatics.GetObjectClass` HitActor) "/Game/Blueprint/BP_GhostPlayer.BP_GhostPlayer_C"))
    (`|SpawnActorFromClass` "/Game/Blueprint/AI/Pawns/BP_FodderGhost.BP_FodderGhost_C" (`KismetMathLibrary.MakeTransform` Location) "Undefined" "OverrideRootScale" null 50.0 null null)
    (`PrimitiveComponent.IgnoreComponentWhenMoving` (`self.RootCollision`) null true))
  (`parent.Destroy` Location HitActor))

(fn `UserConstructionScript`
  (`parent.UserConstructionScript`))