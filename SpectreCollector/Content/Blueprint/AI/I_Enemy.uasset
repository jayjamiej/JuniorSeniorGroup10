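; I_Enemy is a Blueprint interface that defines the shared contract for enemy AI, with references to ghosts, rooms and traps.
; It exposes commands to attack, optionally forced, and to set a target location, plus getters for the ghost, enemy path manager and current room.
; Damage functions toggle and query vulnerability, while separate functions handle stun, sensor and light traps, with the sensor call passing a player.
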(fn `AllowDamage`
  (params (Allow :type Boolean))
  (return))

(fn `Attack`
  (params (Forced :type Boolean)))

(fn `CanBeDamaged`
  (returns (True :type Boolean))
  (return false))

(fn `GetCurrentRoom`
  (returns (Room :type "/Game/Blueprint/RoomManagement/BP_RoomBounds1 Object Reference"))
  (return null))

(fn `GetEnemyPathManager`
  (returns (Manager :type "/Game/Blueprint/AI/Path/BP_GhostPath_Manager Object Reference"))
  (return null))

(fn `GetGhost`
  (returns (Ghost :type "/Game/Blueprint/AI/Pawns/BP_BaseGhost Object Reference"))
  (return null))

(fn `LightTrap`)

(fn `SensorTrap`
  (params (Player :type "Actor Object Reference"))
  (return))

(fn `SetTargetLocation`
  (params (Target :type "Vector Structure")))

(fn `StunTrap`)