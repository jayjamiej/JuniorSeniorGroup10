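; BP_LightTrap is a trap actor that notifies ghosts and furniture when they enter its range.
; DamageSphere records each overlapping actor in a Ghosts array and sends it LightTrapMessage, while FurnitureSphere sends the same message without recording.
; On destruction, the trap sends LightTrapOffMessage to every recorded actor.
; There is no end-overlap handling, so actors stay recorded after leaving, and furniture-only overlaps receive no off message.
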(event `self.DamageSphere.OnComponentBeginOverlap`
  (params (OverlappedComponent :type "PrimitiveComponent Object Reference") (OtherActor :type "Actor Object Reference") (OtherComp :type "PrimitiveComponent Object Reference") (OtherBodyIndex :type Integer) (bFromSweep :type Boolean) (SweepResult :type "HitResult Structure (by ref)"))
  (`KismetArrayLibrary.Array_Add` (`self.Ghosts`) OtherActor)
  (message `/Game/Blueprint/AI/I_Enemy.LightTrap` OtherActor))

(event `self.FurnitureSphere.OnComponentBeginOverlap`
  (params (OverlappedComponent :type "PrimitiveComponent Object Reference") (OtherActor :type "Actor Object Reference") (OtherComp :type "PrimitiveComponent Object Reference") (OtherBodyIndex :type Integer) (bFromSweep :type Boolean) (SweepResult :type "HitResult Structure (by ref)"))
  (message `/Game/Blueprint/AI/I_Enemy.LightTrap` OtherActor))

(event `self.ReceiveDestroyed`
  (for _array_element (`self.Ghosts`)
    (message `/Game/Blueprint/AI/I_Enemy.LightTrapOff` _array_element)))

(fn `UserConstructionScript`
  (`parent.UserConstructionScript`))