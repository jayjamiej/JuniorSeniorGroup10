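; Player controller that routes gamepad input to whatever currently has focus through message calls.
; Init stores the game mode, initializes the controlled pawn's character and creates the HUD.
; GetActiveFocus sends triggers, sticks and buttons to the active UI when it is in the viewport, otherwise to the player character.
; Right-stick axes also drive the HUD crosshair; the stick deadzone checks are left unconnected.
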(event `Init`
  (params (gameMode :type "/Game/Blueprint/BP_GhostGM Object Reference"))
  (set `self.GameMode` gameMode)
  (bind _character (message `/Game/iRef.getPlayerCharacter` (`self.K2_GetPawn`)))
  (bind _output_get (set `self.PlayerCharacter_Ref` _character))
  (`/Game/Blueprint/BP_GhostPlayer.Init` _output_get self)
  (bind _returnvalue (`|CreateWidget` "/Game/Blueprint/UI/UI_PlayerHud.UI_PlayerHud_C"))
  (bind _output_get_2 (set `self.HUD` _returnvalue))
  (`UserWidget.AddToViewport` _output_get_2 0))

(event `InputAction|LeftTrigger`
  (params (Key :type "Key Structure"))
  (bind _focus (`self.GetActiveFocus`))
  (:`Pressed`
    (message `/Game/iController.LeftTrigger_Pressed` _focus))
  (:`Released`
    (message `/Game/iController.LeftTrigger_Released` _focus)))

(event `InputAction|RightTrigger`
  (params (Key :type "Key Structure"))
  (bind _focus (`self.GetActiveFocus`))
  (:`Pressed`
    (message `/Game/iController.RightTrigger_Pressed` _focus))
  (:`Released`
    (message `/Game/iController.RightTrigger_Released` _focus)))

(event `InputAxis|LeftThumb_X`
  (params (AxisValue :type "Float (single-precision)"))
  (message `/Game/iController.LeftThumb` (`self.GetActiveFocus`) (`KismetMathLibrary.MakeVector2D` AxisValue (`self.GetInputAxisValue`))))

(event `InputAction|A`
  (params (Key :type "Key Structure"))
  (:`Pressed`
    (message `/Game/iController.A_Pressed` (`self.GetActiveFocus`))))

(event `InputAxis|LeftThumb_Y`
  (params (AxisValue :type "Float (single-precision)"))
  (message `/Game/iController.LeftThumb` (`self.GetActiveFocus`) (`KismetMathLibrary.MakeVector2D` (`self.GetInputAxisValue`) AxisValue)))

(event `InputAction|B`
  (params (Key :type "Key Structure")))

(event `InputAction|X`
  (params (Key :type "Key Structure")))

(event `InputAction|Y`
  (params (Key :type "Key Structure"))
  (:`Pressed`
    (message `/Game/iController.Y_Pressed` (`self.GetActiveFocus`))))

(event `InputAxis|RightThumb_X`
  (params (AxisValue :type "Float (single-precision)"))
  (message `/Game/iController.RightThumb` (`self.GetActiveFocus`) (`KismetMathLibrary.MakeVector2D` AxisValue (`self.GetInputAxisValue`)))
  (`/Game/Blueprint/UI/UI_PlayerHud.CrosshairRight` (`self.HUD`) AxisValue))

(event `InputAxis|RightThumb_Y`
  (params (AxisValue :type "Float (single-precision)"))
  (message `/Game/iController.RightThumb` (`self.GetActiveFocus`) (`KismetMathLibrary.MakeVector2D` (`self.GetInputAxisValue`) AxisValue))
  (`/Game/Blueprint/UI/UI_PlayerHud.CrosshairDown` (`self.HUD`) AxisValue))

(event `InputAction|LeftStickPress`
  (params (Key :type "Key Structure"))
  (bind _focus (`self.GetActiveFocus`))
  (:`Pressed`
    (message `/Game/iController.Left Stick Press` _focus))
  (:`Released`
    (message `/Game/iController.Left Stick Release` _focus)))

(fn `GetActiveFocus`
  (returns (Focus :type "Object Object Reference"))
  (`/Engine/EditorBlueprintResources/StandardMacros.IsValid` (`self.activeUI`)
    (:`Is Valid`
      (if (`Widget.IsInViewport` (`self.activeUI`))
        (return (`self.activeUI`))
        (else
          (return (`self.PlayerCharacter_Ref`)))))
    (:`Is Not Valid`
      (return (`self.PlayerCharacter_Ref`)))))

(fn `getFurniture`
  (returns (Furniture :type "/Game/Jamie_D/BP_Furniture Object Reference"))
  (return null))

(fn `getPlayerCharacter`
  (returns (Character :type "/Game/Blueprint/BP_GhostPlayer Object Reference"))
  (return null))

(fn `getPlayerController`
  (returns (Controller :type "/Game/Blueprint/BP_PlayerController Object Reference"))
  (return self))

(fn `UserConstructionScript`)