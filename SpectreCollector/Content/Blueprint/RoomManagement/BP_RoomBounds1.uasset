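; Room bounds volume that manages a room's lights, furniture and occupants in a ghost game with a breaker.
; BreakerOn switches lights between saved and off intensities; switching on also damages furniture and makes tracked enemies damageable.
; Entering AI get the room and a random hiding place in their blackboard, recursively avoiding possessed and nearest furniture.
; An entering ghost player triggers a camera change and optionally pauses the Floor's breaker until exit.
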(event `BreakerOn`
  (params (On :type Boolean))
  (bind _rectlightmanager (`self.RectLightManager`))
  (bind _lightvals (`self.LightVals`))
  (set `self.LightOn` On)
  (`/Engine/EditorBlueprintResources/StandardMacros.IsValid` _rectlightmanager
    (:`Is Valid`
      (`/Game/Blueprint/RoomManagement/BP_RectLightManager.LightsActivate` _rectlightmanager (`self.LightOn`)))
    (:`Is Not Valid`
      _))
  (bind _keys (`BlueprintMapLibrary.Map_Keys` _lightvals))
  (for _array_element _keys
    (`LightComponent.SetIntensity` (`Light.LightComponent` _array_element) (select `bool` On :`false` (`self.OffIntensity`) :`true` (`BlueprintMapLibrary.Map_Find` _lightvals _array_element))))
  (if On
    (for _array_element_2 (`self.Furniture`)
      (`GameplayStatics.ApplyDamage` _array_element_2 1.0 null self))
    (for _array_element_3 (`self.EnemyArray`)
      (`/Engine/EditorBlueprintResources/StandardMacros.IsValid` _array_element_3
        (:`Is Valid`
          (message `/Game/Blueprint/AI/I_Enemy.AllowDamage` _array_element_3 true))
        (:`Is Not Valid`
          (`KismetArrayLibrary.Array_RemoveItem` (`self.EnemyArray`) _array_element_3))))))

(event `self.Volume.OnComponentBeginOverlap`
  (params (OverlappedComponent :type "PrimitiveComponent Object Reference") (OtherActor :type "Actor Object Reference") (OtherComp :type "PrimitiveComponent Object Reference") (OtherBodyIndex :type Integer) (bFromSweep :type Boolean) (SweepResult :type "HitResult Structure (by ref)"))
  (bind _returnvalue (`AIBlueprintHelperLibrary.GetAIController` OtherActor))
  (bind _returnvalue_2 (`AIBlueprintHelperLibrary.GetBlackboard` _returnvalue))
  (`KismetSystemLibrary.Delay` 0.2)
  (`/Engine/EditorBlueprintResources/StandardMacros.IsValid` _returnvalue
    (:`Is Valid`
      (message `/Game/Blueprint/AI/I_Enemy.AllowDamage` OtherActor (`self.LightOn`))
      (`KismetArrayLibrary.Array_Add` (`self.EnemyArray`) OtherActor)
      (message `/Game/Blueprint/AI/I_Enemy.SetFloorData` OtherActor self)
      (`/Engine/EditorBlueprintResources/StandardMacros.IsValid` _returnvalue_2
        (:`Is Valid`
          (`BlackboardComponent.SetValueAsObject` _returnvalue_2 "Room" self)
          (bind _closestfurniture (`self.GetClosestFurniture` OtherActor))
          (bind _furniture (`/Game/Blueprint/AI/I_Room.GetRandomFurniture` _closestfurniture true))
          (`BlackboardComponent.SetValueAsObject` _returnvalue_2 "HidingPlace" _furniture))))
    (:`Is Not Valid`
      (if (`KismetMathLibrary.ClassIsChildOf` (`GameplayStatics.GetObjectClass` OtherActor) "/Game/Blueprint/BP_GhostPlayer.BP_GhostPlayer_C")
        (`KismetSystemLibrary.PrintString` "Hello")
        (`self.OnCameraChange` (`self.CameraLength`) (`self.CameraAngle`))
        (if (`self.PausesBreaker`)
          (`/Game/Blueprint/RoomManagement/BP_Floor_Manager.PauseBreaker` (`self.Floor`)))))))

(event `self.Volume.OnComponentEndOverlap`
  (params (OverlappedComponent :type "PrimitiveComponent Object Reference") (OtherActor :type "Actor Object Reference") (OtherComp :type "PrimitiveComponent Object Reference") (OtherBodyIndex :type Integer))
  (if (`KismetMathLibrary.ClassIsChildOf` (`GameplayStatics.GetObjectClass` OtherActor) "/Game/Blueprint/BP_GhostPlayer.BP_GhostPlayer_C")
    (if (`self.PausesBreaker`)
      (`/Game/Blueprint/RoomManagement/BP_Floor_Manager.ResumeBreaker` (`self.Floor`)))
    (else
      (`/Engine/EditorBlueprintResources/StandardMacros.IsValid` (`AIBlueprintHelperLibrary.GetAIController` OtherActor)
        (:`Is Valid`
          (`KismetArrayLibrary.Array_RemoveItem` (`self.EnemyArray`) OtherActor))))))

(event `self.ReceiveBeginPlay`
  (bind _rectlightmanager (`self.RectLightManager`))
  (`/Engine/EditorBlueprintResources/StandardMacros.IsValid` _rectlightmanager
    (:`Is Valid`
      (`/Game/Blueprint/RoomManagement/BP_RectLightManager.Init` _rectlightmanager (`self.OffIntensity`)))
    (:`Is Not Valid`
      _))
  (for _array_element (`self.LightActors`)
    (bind _lightcomponent (`Light.LightComponent` _array_element))
    (bind _intensity (`LightComponentBase.Intensity` _lightcomponent))
    (`KismetSystemLibrary.PrintString` (`KismetStringLibrary.Conv_DoubleToString` _intensity))
    (`BlueprintMapLibrary.Map_Add` (`self.LightVals`) _array_element _intensity)
    (if (not (`self.LightOn`))
      (`LightComponent.SetIntensity` _lightcomponent (`self.OffIntensity`)))))

(event `Init`
  (params (Floor :type "/Game/Blueprint/RoomManagement/BP_Floor_Manager Object Reference"))
  (set `self.Floor` Floor))

(fn `GetClosestFurniture`
  (params (Actor :type "Actor Object Reference"))
  (returns (ClosestFurniture :type "/Game/Jamie_D/BP_Furniture Object Reference"))
  (locals (Closest :type "Float (double-precision)" :default 500000.0) (ClosestActor :type "/Game/Jamie_D/BP_Furniture Object Reference"))
  (bind _furniture (`self.Furniture`))
  (if (!= (`KismetArrayLibrary.Array_Length` _furniture) 0)
    (for _array_element _furniture
      (bind _returnvalue (`KismetMathLibrary.Vector_Distance` (`self.K2_GetActorLocation` _array_element) (`self.K2_GetActorLocation` Actor)))
      (if (< _returnvalue (`local.Closest`))
        (set `local.Closest` _returnvalue)
        (set `local.ClosestActor` _array_element)))
    (return (`local.ClosestActor`))
    (else
      (return null))))

(fn `GetRandomFurniture`
  (params (Previous :type "Actor Object Reference") (NotPossessed :type Boolean))
  (returns (Furniture :type "/Game/Jamie_D/BP_Furniture Object Reference"))
  (locals (LastFurniture :type "Actor Object Reference") (FindEmpty :type Boolean :default false) (Room :type "Array of /Game/Blueprint/RoomManagement/BP_RoomBounds1 Object Reference"))
  (bind _furniture (`self.Furniture`))
  (bind _output (`|GetArrayItem` _furniture))
  (bind _output_2 (`|GetArrayItem` _furniture (`KismetMathLibrary.RandomIntegerInRange` 0 (`KismetArrayLibrary.Array_LastIndex` _furniture))))
  (bind _returnvalue (== _output_2 (`local.LastFurniture`)))
  (set `local.LastFurniture` Previous)
  (if (> (`KismetArrayLibrary.Array_Length` _furniture) 1)
    (bind _output_get (set `local.FindEmpty` NotPossessed))
    (if _output_get
      (if (`/Game/Jamie_D/BP_Furniture.IsPossessed` _output_2)
        _
        (elif _returnvalue
          _
          (else
            (return _output_2))))
      (bind _furniture_2 (`/Game/Blueprint/AI/I_Room.GetRandomFurniture` (`local.LastFurniture`) true))
      (return _furniture_2)
      (elif _returnvalue
        (bind _furniture_3 (`/Game/Blueprint/AI/I_Room.GetRandomFurniture` (`local.LastFurniture`)))
        (return _furniture_3)
        (else
          (return _output_2))))
    (else
      (`/Engine/EditorBlueprintResources/StandardMacros.IsValid` _output
        (:`Is Valid`
          (return _output))))))

(fn `HasFurniture`
  (returns (True :type Boolean))
  (return (> (`KismetArrayLibrary.Array_Length` (`self.Furniture`)) 0)))

(fn `UserConstructionScript`
  (`BoxComponent.SetBoxExtent` (`self.Volume`) (`self.VolumeExtents`) true))