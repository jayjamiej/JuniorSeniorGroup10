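; An interactable breaker switch that temporarily powers its Floor, during which a tooltip says the ghosts are weak and can be dusted.
; Interact passes a DoOnce to animate the switch by timeline, then notifies the Floor, spawns sparks and starts the HUD countdown.
; A timer later calls Reset, which animates the switch again and re-arms the DoOnce.
; Show and hide events toggle the interaction prompt widget.
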(event `Reset`
  (bind _breakertimeon (`self.BreakerTimeOn`))
  (bind (_direction _rotationz) (`Timeline|Timeline_0`)
    (:`Update`
      (`SceneComponent.K2_SetRelativeRotation` (`self.breaker_switch_2`) (`KismetMathLibrary.MakeRotator` _rotationz) false false))
    (:`Finished`
      (goto _label :!via `Reset`))))

(event `/Game/iObjectInteractions.Interact`
  (params (Player :type "/Game/Blueprint/BP_GhostPlayer Object Reference"))
  (bind _breakertimeon (`self.BreakerTimeOn`))
  ;[1 1 1] Activating Breaker
  (`/Engine/EditorBlueprintResources/StandardMacros.DoOnce` false :!label _label
    (:`Completed`
      (bind (_direction _rotationz) (`Timeline|BreakerOn`)
        (:`Update`
          (`SceneComponent.K2_SetRelativeRotation` (`self.breaker_switch_2`) (`KismetMathLibrary.MakeRotator` _rotationz) false false))
        (:`Finished`
          (`/Game/Blueprint/RoomManagement/BP_Floor_Manager.BreakerOn` (`self.Floor`) true (`self.BreakerTimeOn`) (`/Game/Blueprint/BP_GhostPlayer.PlayerController` Player))
          (`self.ToolTipOn`)
          (`GameplayStatics.SpawnEmitterAtLocation` "/Game/Particles/PS_BreakerSpark.PS_BreakerSpark" (+ (`SceneComponent.K2_GetComponentLocation` (`self.StaticMesh`)) (0.0 0.0 50.0)))
          (bind _returnvalue (`KismetSystemLibrary.K2_SetTimerDelegate` (delegate `Reset`) _breakertimeon))
          (`/Game/Blueprint/UI/UI_Timer.StartTimer` (`/Game/Blueprint/UI/UI_PlayerHud.UI_Timer` (`/Game/Blueprint/BP_PlayerController.HUD` (`/Game/Blueprint/BP_GhostPlayer.PlayerController` Player))) _returnvalue _breakertimeon))))))

(event `ToolTipOn`
  (bind _returnvalue (`|CreateWidget` "/Game/UI_ToolTip.UI_ToolTip_C" null "The Ghosts Are Weak And Can Be Dusted!"))
  (bind _output_get (set `self.UIToolTip` _returnvalue))
  (`UserWidget.AddToViewport` _output_get 0)
  (`KismetSystemLibrary.K2_SetTimerDelegate` (delegate `Remove`) 3.0))

(event `Remove`
  (`Widget.RemoveFromParent` (`self.UIToolTip`)))

(event `/Game/iObjectInteractions.ShowInteractionOption`
  ;[1 1 1] Checking if player is in range
  (`SceneComponent.SetVisibility` (`self.Widget`) true false))

(event `/Game/iObjectInteractions.HideInteractionOption`
  ;[1 1 1] Checking if player is in range
  (`SceneComponent.SetVisibility` (`self.Widget`) false false))

(fn `UserConstructionScript`)