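; BP_Floor_Manager manages the rooms on a floor and their breaker-controlled lighting, which affects whether ghosts are vulnerable.
; On BeginPlay it initialises each room with a reference to itself.
; BreakerOn forwards the light state to every room and starts a pausable, resumable timer that calls BreakerOff.
; BreakerOff switches every room off and shows a brief tooltip warning that ghosts are now invulnerable.
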(event `self.ReceiveBeginPlay`
  (for _array_element (`self.Rooms`)
    (`/Game/Blueprint/RoomManagement/BP_RoomBounds1.Init` _array_element self)))

(event `BreakerOn`
  (params (On :type Boolean) (Time :type "Float (double-precision)"))
  ;[1 1 1] Switching lights on in each room
  (for _array_element (`self.Rooms`)
    (`/Game/Blueprint/RoomManagement/BP_RoomBounds1.BreakerOn` _array_element On))
  ;[1 1 1] Breaker Timer management
  (bind _returnvalue (`KismetSystemLibrary.K2_SetTimerDelegate` (delegate `BreakerOff`) Time))
  (set `self.BreakerTimer` _returnvalue))

(event `BreakerOff`
  ;[1 1 1] Breaker Timer management
  (for _array_element (`self.Rooms`)
    (`/Game/Blueprint/RoomManagement/BP_RoomBounds1.BreakerOn` _array_element false))
  (`self.ToolTip`))

(event `PauseBreaker`
  ;[1 1 1] Breaker Timer management
  (`KismetSystemLibrary.K2_PauseTimerHandle` (`self.BreakerTimer`)))

(event `ResumeBreaker`
  ;[1 1 1] Breaker Timer management
  (`KismetSystemLibrary.K2_UnPauseTimerHandle` (`self.BreakerTimer`)))

(event `ToolTip`
  (bind _returnvalue (`|CreateWidget` "/Game/UI_ToolTip.UI_ToolTip_C" null "The Lights Are Off, The Ghost Are Now Invunerable"))
  (bind _output_get (set `self.UIToolTip` _returnvalue))
  (`UserWidget.AddToViewport` _output_get 0)
  (`KismetSystemLibrary.K2_SetTimerDelegate` (delegate `RemoveUI`) 2.0))

(event `RemoveUI`
  (`Widget.RemoveFromParent` (`self.UIToolTip`)))

(fn `UserConstructionScript`)