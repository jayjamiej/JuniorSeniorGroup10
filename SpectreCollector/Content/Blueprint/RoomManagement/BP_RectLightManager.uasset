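; BP_RectLightManager switches a set of rect lights in a room between their original brightness and a shared off intensity.
; BeginPlay caches each light's starting intensity in a map keyed by the light.
; Init scales the supplied off intensity by a multiplier, stores it and applies it to every light.
; LightsActivate restores the cached intensities when on, or applies the stored off intensity when off.
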(event `self.ReceiveBeginPlay`
  (for _array_element (`self.RectLights`)
    (`BlueprintMapLibrary.Map_Add` (`self.Lights`) _array_element (`LightComponentBase.Intensity` (`RectLight.RectLightComponent` _array_element)))))

(event `Init`
  (params (offIntesity :type "Float (double-precision)"))
  (set `self.OffIntensity` (* offIntesity (`self.IntensityMultiplier`)))
  (for _array_element (`self.RectLights`)
    (`LightComponent.SetIntensity` (`RectLight.RectLightComponent` _array_element) (`self.OffIntensity`))))

(event `LightsActivate`
  (params (On :type Boolean))
  (bind _keys (`BlueprintMapLibrary.Map_Keys` (`self.Lights`)))
  (for _array_element _keys
    (`LightComponent.SetIntensity` (`RectLight.RectLightComponent` _array_element) (select `bool` On :`false` (`self.OffIntensity`) :`true` (`BlueprintMapLibrary.Map_Find` (`self.Lights`) _array_element)))))

(fn `UserConstructionScript`)