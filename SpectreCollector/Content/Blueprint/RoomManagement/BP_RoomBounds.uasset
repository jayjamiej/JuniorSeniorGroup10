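; Room volume actor that tracks enemies and furniture and reacts to the ghost player and breaker switching.
; Entering AI join the enemy list and get the room and a random hiding place, recursively re-rolled to avoid possessed or closest furniture, on their blackboard.
; Ghost player entry broadcasts a camera change and swaps walls to a clear material, restored on exit.
; Breaker events set the room light and damage all furniture.
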(event `BreakerOn`
  (params (On :type Boolean))
  (`LightComponent.SetIntensity` (`self.PointLight`) (select `bool` On :`true` (`self.LightIntensity`)))
  (for _array_element (`self.Furniture`)
    (`GameplayStatics.ApplyDamage` _array_element 1.0 null self)))

(event `self.Volume.OnComponentBeginOverlap`
  (params (OverlappedComponent :type "PrimitiveComponent Object Reference") (OtherActor :type "Actor Object Reference") (OtherComp :type "PrimitiveComponent Object Reference") (OtherBodyIndex :type Integer) (bFromSweep :type Boolean) (SweepResult :type "HitResult Structure (by ref)"))
  (bind _returnvalue (`AIBlueprintHelperLibrary.GetAIController` OtherActor))
  (bind _returnvalue_2 (`AIBlueprintHelperLibrary.GetBlackboard` _returnvalue))
  (`KismetSystemLibrary.Delay` 0.2)
  (`/Engine/EditorBlueprintResources/StandardMacros.IsValid` _returnvalue
    (:`Is Valid`
      (`KismetArrayLibrary.Array_Add` (`self.EnemyArray`) OtherActor)
      (`/Engine/EditorBlueprintResources/StandardMacros.IsValid` _returnvalue_2
        (:`Is Valid`
          (`BlackboardComponent.SetValueAsObject` _returnvalue_2 "Room" self)
          (bind _closestfurniture (`self.GetClosestFurniture` OtherActor))
          (bind _furniture (`self.GetRandomFurniture` _closestfurniture true))
          (`BlackboardComponent.SetValueAsObject` _returnvalue_2 "HidingPlace" _furniture))))
    (:`Is Not Valid`
      (if (== (`GameplayStatics.GetObjectClass` OtherActor) "/Game/Blueprint/BP_GhostPlayer.BP_GhostPlayer_C")
        (`self.OnCameraChange` (`self.CameraLength`) (`self.CameraAngle`))
        (for _array_element (`self.WallMeshes`)
          (bind _staticmeshcomponent (`StaticMeshActor.StaticMeshComponent` _array_element))
          (`BlueprintMapLibrary.Map_Add` (`self.WallMaterials`) _array_element (`PrimitiveComponent.GetMaterial` _staticmeshcomponent 0))
          (`PrimitiveComponent.SetMaterial` _staticmeshcomponent 0 "/Game/Blueprint/AI/Wall_ClearMat.Wall_ClearMat"))))))

(event `self.Volume.OnComponentEndOverlap`
  (params (OverlappedComponent :type "PrimitiveComponent Object Reference") (OtherActor :type "Actor Object Reference") (OtherComp :type "PrimitiveComponent Object Reference") (OtherBodyIndex :type Integer))
  (if (== (`GameplayStatics.GetObjectClass` OtherActor) "/Game/Blueprint/BP_GhostPlayer.BP_GhostPlayer_C")
    (for _array_element (`self.WallMeshes`)
      (`PrimitiveComponent.SetMaterial` (`StaticMeshActor.StaticMeshComponent` _array_element) 0 (`BlueprintMapLibrary.Map_Find` (`self.WallMaterials`) _array_element)))
    (else
      (`/Engine/EditorBlueprintResources/StandardMacros.IsValid` (`AIBlueprintHelperLibrary.GetAIController` OtherActor)
        (:`Is Valid`
          (`KismetArrayLibrary.Array_RemoveItem` (`self.EnemyArray`) OtherActor))))))

(fn `GetClosestFurniture`
  (params (Actor :type "Actor Object Reference"))
  (returns (ClosestFurniture :type "/Game/Jamie_D/BP_Furniture Object Reference"))
  (locals (Closest :type "Float (double-precision)" :default 500000.0) (ClosestActor :type "/Game/Jamie_D/BP_Furniture Object Reference"))
  (bind _furniture (`self.Furniture`))
  (if (!= (`KismetArrayLibrary.Array_Length` _furniture) 0)
    (for _array_element _furniture
      (bind _returnvalue (`KismetMathLibrary.Vector_Distance` (`self.K2_GetActorLocation` _array_element) (`self.K2_GetActorLocation` Actor)))
      (if (< _returnvalue (`local.Closest`))
        (set `local.Closest` _returnvalue)
        (set `local.ClosestActor` _array_element)))
    (return (`local.ClosestActor`))
    (else
      (return null))))

(fn `GetRandomFurniture`
  (params (Previous :type "Actor Object Reference") (NotPossessed :type Boolean))
  (returns (Furniture :type "/Game/Jamie_D/BP_Furniture Object Reference"))
  (locals (LastFurniture :type "Actor Object Reference") (FindEmpty :type Boolean :default false))
  (bind _furniture (`self.Furniture`))
  (bind _output (`|GetArrayItem` _furniture (`KismetMathLibrary.RandomIntegerInRange` 0 (`KismetArrayLibrary.Array_LastIndex` _furniture))))
  (bind _returnvalue (== _output (`local.LastFurniture`)))
  (set `local.LastFurniture` Previous)
  (if (!= (`KismetArrayLibrary.Array_Length` _furniture) 0)
    (bind _output_get (set `local.FindEmpty` NotPossessed))
    (if _output_get
      (if (`/Game/Jamie_D/BP_Furniture.IsPossessed` _output)
        _
        (elif _returnvalue
          _
          (else
            (return _output))))
      (bind _furniture_2 (`self.GetRandomFurniture` (`local.LastFurniture`) true))
      (return _furniture_2)
      (elif _returnvalue
        (bind _furniture_3 (`self.GetRandomFurniture` (`local.LastFurniture`)))
        (return _furniture_3)
        (else
          (return _output))))
    (else
      (return null))))

(fn `HasFurniture`
  (returns (True :type Boolean))
  (return (> (`KismetArrayLibrary.Array_Length` (`self.Furniture`)) 0)))

(fn `UserConstructionScript`
  (`BoxComponent.SetBoxExtent` (`self.Volume`) (`self.VolumeExtents`) true))