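; Player character for ghost hunting, with stick movement, a socketed child-actor weapon, ghost dust scoring and overlap-based interaction.
; Left stick input is rotated by a camera yaw snapped to quarter turns, turning the actor and moving it forward.
; BP_GhostDamage uses its damage value as a walk speed multiplier, restored by timer or by collecting dust.
; Controller calls drive weapon fire and interaction through messages to the weapon and overlapped actors.
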(event `Init`
  (params (Controller :type "/Game/Blueprint/BP_PlayerController Object Reference"))
  ;[0 0.522 1] Init
  (set `self.PlayerController` Controller)
  (set `CharacterMovementComponent.MaxWalkSpeed` (`self.baseSpeed`) (`self.CharacterMovement`)))

(event `CollectGhostDust`
  (params (ScoreValue :type Integer))
  ;[0 0.522 1] Functionality to picking up ghost remains
  (`self.ResetSpeedChange`)
  (`/Game/Blueprint/BP_GhostGM.AddScore` (`/Game/Blueprint/BP_PlayerController.GameMode` (`self.PlayerController`)) ScoreValue))

(event `/Game/iController.RightTrigger_Released`
  ;[1 0.1406 0.1406] Weapon Control
  (message `/Game/iObjectInteractions.StopFire` (`ChildActorComponent.ChildActor` (`self.WeaponActor`))))

(event `/Game/iController.RightTrigger_Pressed`
  ;[1 0.1406 0.1406] Weapon Control
  (message `/Game/iObjectInteractions.FireWeapon` (`ChildActorComponent.ChildActor` (`self.WeaponActor`))))

(event `/Game/iController.LeftThumb`
  (params (AxisVector :type "Vector2D Structure"))
  (bind (_returnvalue_roll _returnvalue_pitch _returnvalue_yaw) (`KismetMathLibrary.BreakRotator` (`KismetMathLibrary.ComposeRotators` (`KismetMathLibrary.Conv_VectorToRotator` (`KismetMathLibrary.MakeVector` AxisVector_Y AxisVector_X)) (`self.rotationCamera`))))
  (bind _returnvalue (`KismetMathLibrary.Abs` (`KismetMathLibrary.VSize` (`KismetMathLibrary.MakeVector` AxisVector_X AxisVector_Y))))
  ;[0 0.522 1] Movement Controls
  (if (`self.MovementEnabled`)
    (if (> _returnvalue 0.2)
      (`self.K2_SetActorRotation` (`KismetMathLibrary.MakeRotator` 0.0 0.0 _returnvalue_yaw))
      (`PawnMovementComponent.AddInputVector` (`self.CharacterMovement`) (* (`SceneComponent.GetForwardVector` (`self.Arrow1`)) _returnvalue) false))))

(event `EnableMovement`
  (params (Enabled :type Boolean))
  (set `self.MovementEnabled` Enabled))

(event `self.ReceiveAnyDamage`
  (params (Damage :type "Float (single-precision)") (DamageType :type "DamageType Object Reference") (InstigatedBy :type "Controller Object Reference") (DamageCauser :type "Actor Object Reference"))
  ;[1 0.1406 0.1406] Speed Changing
  (if (== (`GameplayStatics.GetObjectClass` DamageType) "/Game/Blueprint/BP_GhostDamage.BP_GhostDamage_C")
    (if (!= Damage -1.0)
      (bind _output_get (set `self.SpeedMultiplier` Damage :!label _label))
      (`self.SpeedChangeSlow` (* _output_get (`self.baseSpeed`)))
      (bind _returnvalue (`KismetSystemLibrary.K2_SetTimerDelegate` (delegate `BaseSpeedReturn`) 5.0))
      (set `self.speedDebufTimer` _returnvalue)
      (elif (< Damage (`self.SpeedMultiplier`))
        (`KismetSystemLibrary.K2_ClearAndInvalidateTimerHandle` (`self.speedDebufTimer`))
        (goto _label)))))

(event `BaseSpeedReturn`
  ;[1 0.1406 0.1406] Speed Changing
  (`self.ResetSpeedChange`))

(event `/Game/iController.A_Pressed`
  ;[0 0.522 1] Object Interaction
  (`self.InteractWithObjects`))

(event `self.InteractionCollision.OnComponentBeginOverlap`
  (params (OverlappedComponent :type "PrimitiveComponent Object Reference") (OtherActor :type "Actor Object Reference") (OtherComp :type "PrimitiveComponent Object Reference") (OtherBodyIndex :type Integer) (bFromSweep :type Boolean) (SweepResult :type "HitResult Structure (by ref)"))
  ;[0 0.522 1] Object Interaction
  (message `/Game/iObjectInteractions.ShowInteractionOption` OtherActor))

(event `self.InteractionCollision.OnComponentEndOverlap`
  (params (OverlappedComponent :type "PrimitiveComponent Object Reference") (OtherActor :type "Actor Object Reference") (OtherComp :type "PrimitiveComponent Object Reference") (OtherBodyIndex :type Integer))
  ;[0 0.522 1] Object Interaction
  (message `/Game/iObjectInteractions.HideInteractionOption` OtherActor))

(fn `getEnemy`
  (returns (Ghost :type "/Game/Blueprint/BP_BaseGhost Object Reference"))
  (return null))

(fn `getEnemyController`
  (returns (Controller :type "/Game/Blueprint/AI/BP_baseGhostController Object Reference"))
  (return null))

(fn `getFurniture`
  (returns (Furniture :type "/Game/Blueprint/BP_Furniture Object Reference"))
  (return null))

(fn `GetPlayerCharacter`
  (returns (Character :type "/Game/Blueprint/BP_GhostPlayer Object Reference"))
  (return self))

(fn `getPlayerController`
  (returns (Controller :type "/Game/Blueprint/BP_PlayerController Object Reference"))
  (return null))

(fn `InteractWithObjects`
  (for _array_element (`PrimitiveComponent.GetOverlappingActors` (`self.InteractionCollision`) null)
    (message `/Game/iObjectInteractions.Interact` _array_element self)))

(fn `ResetSpeedChange`
  (set `CharacterMovementComponent.MaxWalkSpeed` (`self.baseSpeed`) (`self.CharacterMovement`)))

(fn `SetCameraRotationOffset`
  (params (CameraRotation :type "Rotator Structure"))
  (bind (_remainder _returnvalue) (`KismetMathLibrary.FMod` CameraRotation_Yaw 90.0))
  (set `self.rotationCamera` (`KismetMathLibrary.MakeRotator` 0.0 0.0 (* (select `bool` (>= _remainder 50.0) :`false` _returnvalue :`true` (+ _returnvalue 1)) 90.0))))

(fn `SpeedChangeSlow`
  (params (MaxWalkSpeed :type "Float (double-precision)"))
  (set `CharacterMovementComponent.MaxWalkSpeed` MaxWalkSpeed (`self.CharacterMovement`)))

(fn `UserConstructionScript`
  (`SceneComponent.K2_AttachToComponent` (`self.WeaponActor`) (`self.Mesh`) "WeaponSocket" "KeepRelative" "KeepRelative" "KeepRelative" true))