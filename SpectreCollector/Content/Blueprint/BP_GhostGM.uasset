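; Game mode for a timed, scored Ghost game that quits when the ten-minute timer ends.
; The SpawnDefaultPawnFor override spawns and possesses the pawn without start-spot rotation, passes itself to the controller's message object, then starts the timer and HUD.
; SpawnDefaultPawnAtTransform repeats that spawn and setup at a given transform without starting the game.
; It also stores the latest logged-in player and accumulates score through AddScore.
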(event `StartGame`
  (bind _returnvalue (`KismetSystemLibrary.K2_SetTimerDelegate` (delegate `EndCondition`) 600.0))
  (set `self.Timer` _returnvalue)
  (bind _returnvalue_2 (`|CreateWidget` "/Game/Blueprint/UI/UI_GameHud.UI_GameHud_C" null self))
  (`UserWidget.AddToViewport` _returnvalue_2 0))

(event `EndCondition`
  (`KismetSystemLibrary.QuitGame` (`self.Player`) "Quit"))

(event `self.K2_PostLogin`
  (params (NewPlayer :type "PlayerController Object Reference"))
  (set `self.Player` NewPlayer))

(fn `AddScore`
  (params (ToAdd :type Integer))
  (set `self.Score` (+ (`self.Score`) ToAdd)))

(fn `SpawnDefaultPawnAtTransform`
  (params (NewPlayer :type "Controller Object Reference") (SpawnTransform :type "Transform Structure (by ref)"))
  (returns (ReturnValue :type "Pawn Object Reference"))
  (bind _returnvalue (`|SpawnActorFromClass` (`self.DefaultPawnClass`) (`KismetMathLibrary.MakeTransform` SpawnTransform_Location (struct) SpawnTransform_Scale) "Undefined" "OverrideRootScale" null null))
  (`Controller.Possess` NewPlayer _returnvalue)
  (bind _controller (message `/Game/iRef.getPlayerController` NewPlayer))
  (`/Game/Blueprint/BP_PlayerController.Init` _controller self)
  (return _returnvalue))

(fn `SpawnDefaultPawnFor`
  (params (NewPlayer :type "Controller Object Reference") (StartSpot :type "Actor Object Reference"))
  (returns (ReturnValue :type "Pawn Object Reference"))
  (bind (_returnvalue_location _returnvalue_rotation _returnvalue_scale) (`KismetMathLibrary.BreakTransform` (`self.GetTransform` StartSpot)))
  (bind _returnvalue (`|SpawnActorFromClass` (`self.DefaultPawnClass`) (`KismetMathLibrary.MakeTransform` _returnvalue_location (struct) _returnvalue_scale) "Undefined" "OverrideRootScale" null null))
  (`Controller.Possess` NewPlayer _returnvalue)
  (bind _controller (message `/Game/iRef.getPlayerController` NewPlayer))
  (`/Game/Blueprint/BP_PlayerController.Init` _controller self)
  (`self.StartGame`)
  (return _returnvalue))

(fn `UserConstructionScript`)