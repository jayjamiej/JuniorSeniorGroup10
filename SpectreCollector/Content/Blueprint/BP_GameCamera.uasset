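; BP_GameCamera is a trigger-volume camera that takes over the player's view and tracks them along a spline.
; When a non-ghost player character overlaps the box, it briefly halts and locks their movement while blending the view to this actor.
; Character movement updates then slide the camera's relative X to the closest spline point, leaving other axes unspecified.
; The construction script sizes the box from a configurable extent.
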(event `self.Box.OnComponentBeginOverlap`
  (params (OverlappedComponent :type "PrimitiveComponent Object Reference") (OtherActor :type "Actor Object Reference") (OtherComp :type "PrimitiveComponent Object Reference") (OtherBodyIndex :type Integer) (bFromSweep :type Boolean) (SweepResult :type "HitResult Structure (by ref)"))
  (`KismetSystemLibrary.PrintString` "Hello")
  ;[1 1 1] Overlap
  (if (!= (`GameplayStatics.GetObjectClass` OtherActor) "/Game/Blueprint/BP_BaseGhost.BP_BaseGhost_C")
    (bind _character (message `/Game/iRef.getPlayerCharacter` OtherActor))
    (`/Engine/EditorBlueprintResources/StandardMacros.IsValid` _character
      (:`Is Valid`
        (bind _output_get (set `self.PlayerCharacter` _character))
        (`KismetSystemLibrary.Delay` 0.2)
        (`MovementComponent.StopMovementImmediately` (`Character.CharacterMovement` (`self.PlayerCharacter`)))
        (`/Game/Blueprint/BP_GhostPlayer.EnableMovement` (`self.PlayerCharacter`) false)
        (`PlayerController.SetViewTargetWithBlend` (`/Game/Blueprint/BP_GhostPlayer.PlayerController` _output_get) self 1.0 "VTBlend_Linear" 0.0 false) ; Camera Change
        ;[1 1 1] Setting Camera Rotation
        (bind _character_2 (message `/Game/iRef.getPlayerCharacter` (`self.PlayerCharacter`)))
        (add `Character.OnCharacterMovementUpdated` _character_2 (delegate `MoveCamera`))
        (`KismetSystemLibrary.Delay` 0.5)
        (`/Game/Blueprint/BP_GhostPlayer.EnableMovement` (`self.PlayerCharacter`) true)))))

(event `MoveCamera`
  (params (DeltaSeconds :type "Float (double-precision)") (OldLocation :type "Vector Structure") (OldVelocity :type "Vector Structure"))
  (bind _returnvalue_location (`KismetMathLibrary.BreakTransform` (`self.GetTransform` (`self.PlayerCharacter`))))
  (bind _returnvalue_x (`KismetMathLibrary.BreakVector` (`SplineComponent.FindLocationClosestToWorldLocation` (`self.Spline`) _returnvalue_location "Local")))
  (`SceneComponent.K2_SetRelativeLocation` (`self.Camera`) (`KismetMathLibrary.MakeVector` _returnvalue_x) false false))

(fn `UserConstructionScript`
  (`BoxComponent.SetBoxExtent` (`self.Box`) (`self.BoxExtent`) true))