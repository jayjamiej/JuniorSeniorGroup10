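; BP_testplayer is a test player Blueprint that detects lifts and publishes its position to materials.
; Overlapping an actor tagged "Lift" stores it as LiftManager and hands it to the PlayerController through GetLiftManager.
; After the parent Tick, it writes the capsule and camera world locations into the PlayerLocation Material Parameter Collection every frame, making both available to shaders.
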(event `self.ReceiveActorBeginOverlap`
  (params (OtherActor :type "Actor Object Reference"))
  (if (`self.ActorHasTag` OtherActor "Lift")
    (bind _output_get (set `self.Lift Manager` OtherActor))
    (`/Game/Blueprint/BP_PlayerController.GetLiftManager` (`self.PlayerController`) _output_get)))

(event `self.ReceiveTick`
  (params (DeltaSeconds :type "Float (single-precision)"))
  (`parent.ReceiveTick` DeltaSeconds)
  (`KismetMaterialLibrary.SetVectorParameterValue` "/Game/Jamie_D/Shaders/PlayerLocation.PlayerLocation" "Location" (`KismetMathLibrary.Conv_VectorToLinearColor` (`SceneComponent.K2_GetComponentLocation` (`self.CapsuleComponent`))))
  (`KismetMaterialLibrary.SetVectorParameterValue` "/Game/Jamie_D/Shaders/PlayerLocation.PlayerLocation" "CameraLocation" (`KismetMathLibrary.Conv_VectorToLinearColor` (`SceneComponent.K2_GetComponentLocation` (`self.Camera`)))))

(fn `UserConstructionScript`
  (`parent.UserConstructionScript`))