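; BP_Weapon is a spotlight weapon that alternates between a ghost search mode and a damaging fire mode.
; Searching uses a looping timer to toggle the Capsule component's active state.
; Firing stops the search, animates the spotlight cone through a timeline and repeatedly sphere-traces forward to damage the hit actor.
; Stopping fire resets the cone and resumes searching; older furniture-detection traces and light toggles remain unconnected.
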(event `/Game/iObjectInteractions.StopFire`
  ;[1 1 1] Weapon Firing+LineTrace
  (`self.Init Weapon`)
  ;;[1 1 1] Set Outer Cone Angle
  (`SpotLightComponent.SetOuterConeAngle` (`self.SpotLight`) 20.0)
  (`KismetSystemLibrary.K2_ClearAndInvalidateTimerHandle` (`self.ShootingTimer`)))

(event `/Game/iObjectInteractions.FireWeapon`
  ;[1 1 1] Weapon Firing+LineTrace
  (`KismetSystemLibrary.K2_ClearAndInvalidateTimerHandle` (`self.Searching`))
  (bind _returnvalue (`KismetSystemLibrary.K2_SetTimerDelegate` (delegate `Shooting`) 0.25 true))
  (set `self.ShootingTimer` _returnvalue)
  ;;[1 1 1] Set Outer Cone Angle
  (bind (_direction _outerconeangle) (`Timeline|Radius` :!via `PlayFromStart`)
    (:`Update`
      (`SpotLightComponent.SetOuterConeAngle` (`self.SpotLight`) _outerconeangle))))

(event `Shooting`
  (bind _arrow (`self.Arrow`))
  (bind _returnvalue (`SceneComponent.K2_GetComponentLocation` _arrow))
  ;[1 1 1] Weapon Firing+LineTrace
  (bind _outhit (`KismetSystemLibrary.SphereTraceSingle` :`Start` _returnvalue :`End` (+ _returnvalue (* (`SceneComponent.GetForwardVector` _arrow) 500.0)) :`Radius` 35.0 :`TraceChannel` "TraceTypeQuery1" :`DrawTime` 1.0))
  (`GameplayStatics.ApplyDamage` (`.HitActor` (`GameplayStatics.BreakHitResult` _outhit)) (`self.damageAmount`)))

(event `self.Init Weapon`
  ;[1 1 1] Weapon Ghost Search
  (bind _returnvalue (`KismetSystemLibrary.K2_SetTimerDelegate` (delegate `Search`) 0.1 true))
  (set `self.Searching` _returnvalue))

(event `Search`
  ;[1 1 1] Weapon Ghost Search
  (`ActorComponent.ToggleActive` (`self.Capsule`)))

(fn `UserConstructionScript`)