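; BP_GameCamera is a placed camera actor that takes over the player's view when an actor enters its trigger box.
; On overlap it waits briefly, then gets the overlapping actor's instigator controller and blends that player controller's view target to itself.
; The construction script sets the spring arm's yaw and the trigger box extent from variables, so each placed camera can be configured.
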(event `self.Box.OnComponentBeginOverlap`
  (params (OverlappedComponent :type "PrimitiveComponent Object Reference") (OtherActor :type "Actor Object Reference") (OtherComp :type "PrimitiveComponent Object Reference") (OtherBodyIndex :type Integer) (bFromSweep :type Boolean) (SweepResult :type "HitResult Structure (by ref)"))
  (bind _output_get (set `self.PlayerCharacter` OtherActor))
  (`KismetSystemLibrary.Delay` 0.2)
  (bind _returnvalue (`self.GetInstigatorController` _output_get))
  (`/Engine/EditorBlueprintResources/StandardMacros.IsValid` _returnvalue
    (:`Is Valid`
      (bind _controller (message `/Game/iRef.getPlayerController` _returnvalue))
      (`/Engine/EditorBlueprintResources/StandardMacros.IsValid` _controller
        (:`Is Valid`
          (`PlayerController.SetViewTargetWithBlend` _controller self 0.0 "VTBlend_Linear" 0.0 false))))))

(fn `UserConstructionScript`
  (`SceneComponent.K2_SetRelativeRotation` (`self.SpringArm`) (`KismetMathLibrary.MakeRotator` 0.0 0.0 (`self.Z-Axis`)) false false)
  (`BoxComponent.SetBoxExtent` (`self.Box`) (`self.NewVar_0`) true))