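; Game mode for the ghost game that runs a timed session and keeps the score.
; SpawnDefaultPawnFor spawns and possesses the pawn at the start spot, passes itself to the player controller through Init, then calls StartGame.
; StartGame creates the TestHUD with a game mode reference and starts a one-shot timer that quits the game for the player stored in PostLogin.
; AddScore accumulates points into Score.
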(event `StartGame`
  (bind _returnvalue (`KismetSystemLibrary.K2_SetTimerDelegate` (delegate `EndCondition`) 600.0))
  (set `self.Timer` _returnvalue)
  (bind _returnvalue_2 (`|CreateWidget` "/Game/Blueprint/TestHUD.TestHUD_C" null self))
  (`UserWidget.AddToViewport` _returnvalue_2 0))

(event `EndCondition`
  (`KismetSystemLibrary.QuitGame` (`self.Player`) "Quit"))

(event `self.K2_PostLogin`
  (params (NewPlayer :type "PlayerController Object Reference"))
  (set `self.Player` NewPlayer))

(fn `AddScore`
  (params (ToAdd :type Integer))
  (set `self.Score` (+ (`self.Score`) ToAdd)))

(fn `SpawnDefaultPawnFor`
  (params (NewPlayer :type "Controller Object Reference") (StartSpot :type "Actor Object Reference"))
  (returns (ReturnValue :type "Pawn Object Reference"))
  (bind _returnvalue (`|SpawnActorFromClass` (`self.DefaultPawnClass`) (`self.GetTransform` StartSpot) "Undefined" "OverrideRootScale" null null))
  (`Controller.Possess` NewPlayer _returnvalue)
  (bind _controller (message `/Game/iRef.getPlayerController` NewPlayer))
  (`/Game/Blueprint/BP_PlayerController.Init` _controller self)
  (`self.StartGame`)
  (return _returnvalue))

(fn `UserConstructionScript`)