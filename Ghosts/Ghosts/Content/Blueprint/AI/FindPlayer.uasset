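; FindPlayer is a behavior tree service that looks for a player character near the AI's pawn and stores it as the blackboard target.
; On search start it clears Target, then runs a near-stationary sphere trace for Pawn objects around the controlled pawn using SearchRadius.
; The single hit actor receives a GetPlayerCharacter interface message, and a valid result is written to Target.
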(event `self.ReceiveSearchStartAI`
  (params (OwnerController :type "AIController Object Reference") (ControlledPawn :type "Pawn Object Reference"))
  (bind _returnvalue (`Actor.K2_GetActorLocation` ControlledPawn))
  (`BTFunctionLibrary.SetBlackboardValueAsObject` (`self.Target`))
  (`/Engine/EditorBlueprintResources/StandardMacros.IsValid` ControlledPawn
    (:`Is Valid`
      (bind _outhit (`KismetSystemLibrary.SphereTraceSingleForObjects` _returnvalue (+ _returnvalue (0.0 0.0 1.0)) (`self.SearchRadius`) (`|MakeArray` "ObjectTypeQuery3" :!type "EObjectTypeQuery Enum")))
      (bind (_bblockinghit _binitialoverlap _time _distance _location _impactpoint _normal _impactnormal _physmat _hitactor) (`GameplayStatics.BreakHitResult` _outhit))
      (if _bblockinghit
        (bind _character (message `/Game/iRef.getPlayerCharacter` _hitactor))
        (`/Engine/EditorBlueprintResources/StandardMacros.IsValid` _character
          (:`Is Valid`
            (`BTFunctionLibrary.SetBlackboardValueAsObject` (`self.Target`) _character)))))))