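; Behavior tree service that, on search start, picks a hiding piece of furniture for a ghost AI.
; It gets the Ghost from the controlled pawn, stores a chosen BP_Furniture in the Furniture blackboard key and sets IsHiding.
; FindUnpossessed recursively retries random picks, aiming for unpossessed furniture outside the ghost's spawn room.
; The random index is a pure node evaluated separately per use, so the returned piece can differ from those checked.
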(event `self.ReceiveSearchStartAI`
  (params (OwnerController :type "AIController Object Reference") (ControlledPawn :type "Pawn Object Reference"))
  (bind _ghost (message `/Game/iRef.getEnemy` ControlledPawn))
  (set `self.Ghost` _ghost)
  (`BTFunctionLibrary.SetBlackboardValueAsObject` (`self.Furniture`))
  (bind _output (`self.FindUnpossessed`))
  (`BTFunctionLibrary.SetBlackboardValueAsObject` (`self.Furniture`) _output)
  (`BTFunctionLibrary.SetBlackboardValueAsBool` (`self.IsHiding`) true))

(fn `FindUnpossessed`
  (returns (Output :type "/Game/Blueprint/BP_Furniture Object Reference"))
  (bind _outactors (`GameplayStatics.GetAllActorsOfClass` "/Game/Blueprint/BP_Furniture.BP_Furniture_C"))
  (bind _output (`|GetArrayItem` _outactors (`KismetMathLibrary.RandomIntegerInRange` 0 (`KismetArrayLibrary.Array_LastIndex` _outactors))))
  (if (`/Game/Blueprint/BP_Furniture.IsPossessed` _output)
    _
    (elif (`KismetStringLibrary.EqualEqual_StrStr` (`KismetSystemLibrary.GetDisplayName` (`/Game/Blueprint/BP_Furniture.Room` _output)) (`KismetSystemLibrary.GetDisplayName` (`/Game/Blueprint/BP_BaseGhost.SpawnRoom` (`self.Ghost`))))
      _
      (else
        (return _output))))
  (bind _output_2 (`self.FindUnpossessed`))
  (return _output_2))