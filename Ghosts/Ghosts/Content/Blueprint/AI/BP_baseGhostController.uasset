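; Base AI controller for ghost enemies that starts their behavior on BeginPlay.
; It runs the Ghostbasic behavior tree, then initializes the IsHiding blackboard key to false.
; A set of getter functions covers enemy, furniture, player and controller lookups; only GetEnemyController returns a value (itself), while the rest are empty.
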(event `self.ReceiveBeginPlay`
  (`self.RunBehaviorTree` "/Game/Blueprint/AI/Ghostbasic.Ghostbasic")
  (`BlackboardComponent.SetValueAsBool` (`AIBlueprintHelperLibrary.GetBlackboard` null) "IsHiding" false))

(fn `getEnemy`
  (returns (Ghost :type "/Game/Blueprint/BP_BaseGhost Object Reference"))
  (return null))

(fn `getEnemyController`
  (returns (Controller :type "/Game/Blueprint/AI/BP_baseGhostController Object Reference"))
  (return self))

(fn `getFurniture`
  (returns (Furniture :type "/Game/Blueprint/BP_Furniture Object Reference"))
  (return null))

(fn `getPlayerCharacter`
  (returns (Character :type "/Game/Blueprint/BP_GhostPlayer Object Reference"))
  (return null))

(fn `getPlayerController`
  (returns (Controller :type "/Game/Blueprint/BP_PlayerController Object Reference"))
  (return null))

(fn `UserConstructionScript`)