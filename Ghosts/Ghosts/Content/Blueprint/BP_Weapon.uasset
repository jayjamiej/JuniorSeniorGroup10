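; BP_Weapon is a hitscan weapon Blueprint that damages whatever actor its line trace hits.
; FireWeapon immediately runs a short Visibility trace along the Arrow component's forward vector, with persistent debug drawing, and applies DamageAmount to the hit actor without checking the hit result.
; The same sequence starts a FireRate delay that calls StopFireMessage when it ends.
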(event `/Game/iObjectInteractions.FireWeapon`
  (bind _arrow (`self.Arrow`))
  (bind _returnvalue (`SceneComponent.K2_GetComponentLocation` _arrow))
  ;[1 1 1] Weapon Firing+LineTrace
  (`|ExecutionSequence`
    (:`then_0`
      (`KismetSystemLibrary.Delay` (`self.fireRate`))
      (message `/Game/iObjectInteractions.StopFire` self))
    (:`then_1`
      (bind _outhit (`KismetSystemLibrary.LineTraceSingle` :`Start` _returnvalue :`End` (+ _returnvalue (* (`SceneComponent.GetForwardVector` _arrow) 500.0)) :`TraceChannel` "TraceTypeQuery1" :`DrawDebugType` "Persistent"))
      (`GameplayStatics.ApplyDamage` (`.HitActor` (`GameplayStatics.BreakHitResult` _outhit)) (`self.damageAmount`)))))

(fn `UserConstructionScript`)