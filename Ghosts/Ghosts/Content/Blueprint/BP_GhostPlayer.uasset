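; BP_GhostPlayer is a ghost player character that moves with a thumbstick and fires an attached weapon.
; Left-stick input past a small deadzone sets yaw to the stick direction and adds movement along the arrow's forward, scaled by deflection.
; Right-trigger press and release send fire and stop messages to the WeaponActor child actor, attached to the mesh's WeaponSocket at construction.
; GetPlayerCharacter returns itself, while GetPlayerController returns nothing.
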(event `/Game/iController.RightTrigger_Released`
  (message `/Game/iObjectInteractions.StopFire` (`ChildActorComponent.ChildActor` (`self.WeaponActor`))))

(event `/Game/iController.RightTrigger_Pressed`
  (message `/Game/iObjectInteractions.FireWeapon` (`ChildActorComponent.ChildActor` (`self.WeaponActor`))))

(event `/Game/iController.LeftThumb`
  (params (AxisVector :type "Vector2D Structure"))
  (bind (_returnvalue_roll _returnvalue_pitch _returnvalue_yaw) (`KismetMathLibrary.BreakRotator` (`KismetMathLibrary.Conv_VectorToRotator` (`KismetMathLibrary.MakeVector` AxisVector_Y AxisVector_X))))
  (bind _returnvalue (`KismetMathLibrary.Abs` (`KismetMathLibrary.VSize` (`KismetMathLibrary.MakeVector` AxisVector_X AxisVector_Y))))
  (if (> _returnvalue 0.2)
    (`self.K2_SetActorRotation` (`KismetMathLibrary.MakeRotator` 0.0 0.0 _returnvalue_yaw))
    (`PawnMovementComponent.AddInputVector` (`self.CharacterMovement`) (* (`SceneComponent.GetForwardVector` (`self.Arrow1`)) _returnvalue) false)))

(fn `GetPlayerCharacter`
  (returns (Character :type "/Game/Blueprint/BP_GhostPlayer Object Reference"))
  (return self))

(fn `getPlayerController`
  (returns (Controller :type "/Game/Blueprint/BP_PlayerController Object Reference"))
  (return null))

(fn `UserConstructionScript`
  (`SceneComponent.K2_AttachToComponent` (`self.WeaponActor`) (`self.Mesh`) "WeaponSocket" "KeepRelative" "KeepRelative" "KeepRelative" true))