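; BP_BaseGhost is a base ghost actor that can be damaged and leaves a pickup behind when it dies.
; AnyDamage passes incoming damage to a Damage function that subtracts it from Health.
; When Health reaches zero or below, it always spawns the PickUp class at the Plane component's world transform, then calls Death, which destroys the actor.
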(event `self.ReceiveAnyDamage`
  (params (Damage :type "Float (single-precision)") (DamageType :type "DamageType Object Reference") (InstigatedBy :type "Controller Object Reference") (DamageCauser :type "Actor Object Reference"))
  (`self.Damage` Damage)
  (if (<= (`self.Health`) 0.0)
    (`|SpawnActorFromClass` "/Game/Blueprint/PickUp.PickUp_C" (`SceneComponent.K2_GetComponentToWorld` (`self.Plane`)) "AlwaysSpawn" "OverrideRootScale" null null)
    (`self.Death`)))

(fn `Damage`
  (params (Damage :type "Float (double-precision)"))
  (set `self.Health` (- (`self.Health`) Damage)))

(fn `Death`
  (`self.K2_DestroyActor`))

(fn `UserConstructionScript`
  (`parent.UserConstructionScript`))