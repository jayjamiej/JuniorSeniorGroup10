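; Furniture actor that ghosts can possess and the player can interact with to force the ghost back out.
; A hiding ghost overlapping the sphere is destroyed, saving its class and health; GhostStartPoint furniture instead starts possessed at max health.
; While possessed, an effect plays and a looping timer rocks the mesh.
; Interacting, prompted by a widget, respawns the ghost with its stored health.
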(event `self.ReceiveBeginPlay`
  (if (`self.GhostStartPoint`)
    (`self.Possess` null)))

(event `Possess`
  (params (Ghost :type "/Game/Blueprint/BP_BaseGhost Object Reference"))
  (`/Engine/EditorBlueprintResources/StandardMacros.IsValid` Ghost
    (:`Is Valid`
      (set `self.GhostStats` (make `/Game/Blueprint/sGhostStats` (`/Game/Blueprint/BP_BaseGhost.Health` Ghost)))
      (set `self.GhostClass` (`GameplayStatics.GetObjectClass` Ghost))
      (`self.K2_DestroyActor` Ghost)
      (set `self.IsPossessed` true :!label _label)
      (`ActorComponent.Activate` (`self.Possession`) false)
      (bind _returnvalue (`KismetSystemLibrary.K2_SetTimerDelegate` (delegate `PossessAnim`) 2.0 true))
      (set `self.AnimTimer` _returnvalue))
    (:`Is Not Valid`
      (if (`self.GhostStartPoint`)
        (set `self.GhostStats` (make `/Game/Blueprint/sGhostStats` (`.maxHealth` (defaults `/Game/Blueprint/BP_Furniture` (`self.GhostClass`)))))
        (goto _label)))))

(event `PossessAnim`
  (bind (_direction _alpha) (`Timeline|Anim` :!via `PlayFromStart`)
    (:`Update`
      (`SceneComponent.K2_SetRelativeRotation` (`self.Mesh`) (`KismetMathLibrary.RLerp` (struct :`Roll` 15.0) (struct :`Roll` -15.0) _alpha) false false))))

(event `/Game/iObjectInteractions.Interact`
  (params (Player :type "/Game/Blueprint/BP_GhostPlayer Object Reference"))
  (if (`self.IsPossessed`)
    (`KismetSystemLibrary.K2_ClearAndInvalidateTimerHandle` (`self.AnimTimer`))
    (`ActorComponent.Deactivate` (`self.Possession`))
    (set `self.IsPossessed` false)
    (`|SpawnActorFromClass` (`self.GhostClass`) (`SceneComponent.K2_GetComponentToWorld` (`self.SpawnLocation`)) "Undefined" "OverrideRootScale" null (`.Health_3_E06504AE4EF0129E5278D0B603BB5944` (break `/Game/Blueprint/sGhostStats` (`self.GhostStats`))) (`self.Room`) null)
    (`SceneComponent.SetVisibility` (`self.Widget`) false false)))

(event `/Game/iObjectInteractions.ShowInteractionOption`
  (if (`self.IsPossessed`)
    (`SceneComponent.SetVisibility` (`self.Widget`) true false)))

(event `/Game/iObjectInteractions.HideInteractionOption`
  (`SceneComponent.SetVisibility` (`self.Widget`) false false))

(event `self.GhostOverlap.OnComponentBeginOverlap`
  (params (OverlappedComponent :type "PrimitiveComponent Object Reference") (OtherActor :type "Actor Object Reference") (OtherComp :type "PrimitiveComponent Object Reference") (OtherBodyIndex :type Integer) (bFromSweep :type Boolean) (SweepResult :type "HitResult Structure (by ref)"))
  (bind _ghost (message `/Game/iRef.getEnemy` OtherActor))
  (`/Engine/EditorBlueprintResources/StandardMacros.IsValid` _ghost
    (:`Is Valid`
      (bind _controller (message `/Game/iRef.getEnemyController` (`Pawn.GetController` _ghost)))
      (`/Engine/EditorBlueprintResources/StandardMacros.IsValid` _controller
        (:`Is Valid`
          (if (`BlackboardComponent.GetValueAsBool` (`AIBlueprintHelperLibrary.GetBlackboard` _controller) "IsHiding")
            (`self.Possess` _ghost)))))))

(fn `getEnemy`
  (returns (Ghost :type "/Game/Blueprint/BP_BaseGhost Object Reference"))
  (return null))

(fn `getEnemyController`
  (returns (Controller :type "/Game/Blueprint/AI/BP_baseGhostController Object Reference"))
  (return null))

(fn `getFurniture`
  (returns (Furniture :type "/Game/Blueprint/BP_Furniture Object Reference"))
  (return self))

(fn `getPlayerCharacter`
  (returns (Character :type "/Game/Blueprint/BP_GhostPlayer Object Reference"))
  (return null))

(fn `getPlayerController`
  (returns (Controller :type "/Game/Blueprint/BP_PlayerController Object Reference"))
  (return null))

(fn `UserConstructionScript`
  (bind _mesh (`self.Mesh`))
  (`BoxComponent.SetBoxExtent` (`self.Root`) (`self.RootCollisionExtents`) true)
  (`StaticMeshComponent.SetStaticMesh` _mesh (`self.FurnitureMesh`))
  (`SceneComponent.K2_SetRelativeLocation` _mesh (`self.MeshOffset`) false false)
  (`SphereComponent.SetSphereRadius` (`self.GhostOverlap`) (`self.SphereRadius`) true))