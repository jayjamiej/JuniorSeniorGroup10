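; BP_GhostPlayer is a player-controlled character that moves with the left thumbstick and fires a weapon with the right trigger.
; Stick input feeds CharacterMovement along the actor's forward vector and a 90-degree rotated copy of it for strafing.
; Pulling the trigger past halfway sends a fire message to the WeaponActor child actor through a DoOnce, which resets on release for one shot per pull.
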(event `InputAxis|LeftThumb_Y`
  (params (AxisValue :type "Float (single-precision)"))
  (`PawnMovementComponent.AddInputVector` (`self.CharacterMovement`) (* (`self.GetActorForwardVector`) AxisValue) false))

(event `InputAxis|LeftThumb_X`
  (params (AxisValue :type "Float (single-precision)"))
  (`PawnMovementComponent.AddInputVector` (`self.CharacterMovement`) (* (`KismetMathLibrary.GreaterGreater_VectorRotator` (`self.GetActorForwardVector`) (struct :`Yaw` 90.0)) AxisValue) false))

(event `InputAxis|RightTrigger`
  (params (AxisValue :type "Float (single-precision)"))
  (if (> AxisValue 0.5)
    (`/Engine/EditorBlueprintResources/StandardMacros.DoOnce` false :!label _label
      (:`Completed`
        (message `/Game/iObjectInteractions.FireWeapon` (`ChildActorComponent.ChildActor` (`self.WeaponActor`)))))
    (else
      (goto _label :!via `Reset`))))

(fn `UserConstructionScript`)